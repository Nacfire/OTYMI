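; Console_Light is an indicator light that shows red or green on a sphere mesh, likely for a console.
; The construction script creates a dynamic instance of the assigned material, if valid, and applies it to the sphere.
; The On event sets its Base Color parameter to red.
; The Green event sets it to green, then switches it to black after a one-second delay.
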(event Custom|On
  (Rendering|Material|SetVectorParameterValue (Variables|Default|GetDynMat) "Base Color" "(R=1.000000,G=0.006871,B=0.000000,A=1.000000)" :!class /Script/Engine.MaterialInstanceDynamic))

(event Custom|Green
  (Rendering|Material|SetVectorParameterValue (Variables|Default|GetDynMat) "Base Color" "(R=0.005746,G=1.000000,B=0.000000,A=1.000000)" :!class /Script/Engine.MaterialInstanceDynamic)
  (Utilities|FlowControl|Delay 1.0)
  (Rendering|Material|SetVectorParameterValue (Variables|Default|GetDynMat) "Base Color" "(R=0.000000,G=0.000000,B=0.000000,A=1.000000)" :!class /Script/Engine.MaterialInstanceDynamic))

(event EventBeginPlay)

(event Collision|EventActorBeginOverlap
  (params (OtherActor :type Actor%20Object%20Reference)))

(event EventTick
  (params (DeltaSeconds :type Float%20%28single-precision%29)))

(fn ConstructionScript
  (Variables|Default|GetMaterial
    (:then
      (bind _returnvalue (Rendering|Material|CreateDynamicMaterialInstance (Variables|Default|GetSphere) 0 (Variables|Default|GetMaterial) "None" :!class /Script/Engine.PrimitiveComponent))
      (bind _output_get (Variables|Default|SetDynMat _returnvalue))
      (Rendering|Material|SetMaterial (Variables|Default|GetSphere) 0 _output_get))
    (:else)))