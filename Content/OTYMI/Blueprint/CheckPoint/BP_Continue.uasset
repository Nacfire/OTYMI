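; BP_Continue restores the level from the checkpoint stored in GI_CheckPoint at BeginPlay.
; With an active checkpoint, it repositions "Saved"-tagged actors by array index, restarts looping platforms and disconnect zones, and restores camera spline points, pivot rotations and rotation-trigger flags.
; It also moves the Multiprise and each player, matched by PlayerID, to saved locations.
; Otherwise, it passes starting player, Multiprise, pivot and spline references to the game instance.
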(event EventBeginPlay
  (bind _asgi_check_point (Utilities|Casting|CastToGI_CheckPoint (Game|GetGameInstance)))
  (Variables|Default|SetAs%20GI%20Check%20Point _asgi_check_point)
  (if (Variables|/Game/OTYMI/Blueprint/CheckPoint/GI_CheckPoint.GI_CheckPoint_C|GetbIsCheckPointActive _asgi_check_point)
    (bind _outactors (Actor|GetAllActorswithTag "Saved"))
    (for (_array_element _array_index) _outactors
      (Transformation|SetActorTransform _array_element (Utilities|Array|Get(acopy) (Variables|/Game/OTYMI/Blueprint/CheckPoint/GI_CheckPoint.GI_CheckPoint_C|GetLocation%20Objet%20Saved (Variables|Default|GetAs%20GI%20Check%20Point)) _array_index))
      (bind _asbp_disconect__zone_mobil (Utilities|Casting|CastToBP_Disconect-Zone_Mobil _array_element)
        (:then
          (if (Variables|/Game/OTYMI/Blueprint/BP_Disconect-Zone_Mobil.BP_Disconect-Zone_Mobil_C|GetLoop _asbp_disconect__zone_mobil)
            (Default|PlayStartOpen _asbp_disconect__zone_mobil)))
        (:CastFailed
          (bind _asbp_platforme_mobil (Utilities|Casting|CastToBP_PlatformeMobil _array_element)
            (:then
              (if (Variables|/Game/OTYMI/Buton_et_interactible/BP_PlatformeMobil.BP_PlatformeMobil_C|GetLoop _asbp_platforme_mobil)
                (Default|PlayStartOpen _asbp_platforme_mobil)))
            (:CastFailed
              (bind _asbp_platforme_rotate (Utilities|Casting|CastToBP_PlatformeRotate _array_element))
              (if (Variables|/Game/OTYMI/Buton_et_interactible/BP_PlatformeRotate.BP_PlatformeRotate_C|GetLoop _asbp_platforme_rotate)
                (Default|PlayStartOpen _asbp_platforme_rotate)))))))
    (for (_array_element_2 _array_index_2) (Variables|/Game/OTYMI/Blueprint/CheckPoint/GI_CheckPoint.GI_CheckPoint_C|GetLocationPointSpline (Variables|Default|GetAs%20GI%20Check%20Point))
      (Variables|Default|SetArray%20Element_0 _array_element_2)
      (Variables|Default|SetArray%20Index _array_index_2)
      (Spline|SetLocationatSplinePoint (Variables|/Game/OTYMI/Blueprint/Bp_CameraSpline.Bp_CameraSpline_C|GetCam%20Spline (Variables|Default|GetCamSpline)) (Variables|Default|GetArray%20Index) (Variables|Default|GetArray%20Element_0) "Local" true))
    (Variables|/Game/OTYMI/Blueprint/BP_MovePointOnCameraSpline.BP_MovePointOnCameraSpline_C|SetActivate (Variables|Default|Getmove%20point%20spline) (Variables|/Game/OTYMI/Blueprint/CheckPoint/GI_CheckPoint.GI_CheckPoint_C|GetPoint%20Spline%20Move? (Variables|Default|GetAs%20GI%20Check%20Point)))
    (for (_array_element_3 _array_index_3) (Variables|Default|GetPivot%20Ref)
      (Transformation|SetActorRotation _array_element_3 (Utilities|Array|Get(acopy) (Variables|/Game/OTYMI/Blueprint/CheckPoint/GI_CheckPoint.GI_CheckPoint_C|GetRotationPivot (Variables|Default|GetAs%20GI%20Check%20Point)) _array_index_3) true))
    (for _array_element_4 (Variables|Default|GetTriggertRotationEnviro)
      (bind _asbp_rotation_salon_ld1to_ld2 (Utilities|Casting|CastToBP_Rotation_Salon_LD1ToLD2 _array_element_4)
        (:then
          (Variables|/Game/OTYMI/Blueprint/BP_Rotation_Salon_LD1ToLD2.BP_Rotation_Salon_LD1ToLD2_C|SetDid%20Turn%20? _asbp_rotation_salon_ld1to_ld2 (Variables|/Game/OTYMI/Blueprint/CheckPoint/GI_CheckPoint.GI_CheckPoint_C|GetDid%20Turn%20?LR1-2 (Variables|Default|GetAs%20GI%20Check%20Point))))
        (:CastFailed
          (bind _asbp_rotation_salon_ld2to_ld3 (Utilities|Casting|CastToBP_Rotation_Salon_LD2ToLD3 _array_element_4)
            (:then
              (Variables|/Game/OTYMI/Blueprint/BP_Rotation_Salon_LD2ToLD3.BP_Rotation_Salon_LD2ToLD3_C|SetDid%20Turn%20? _asbp_rotation_salon_ld2to_ld3 (Variables|/Game/OTYMI/Blueprint/CheckPoint/GI_CheckPoint.GI_CheckPoint_C|GetDid%20Turn%20?LR2-3 (Variables|Default|GetAs%20GI%20Check%20Point))))
            (:CastFailed
              (bind _asbp_rotation_kitchen_ld1to_ld2 (Utilities|Casting|CastToBP_Rotation_Kitchen_LD1ToLD2 _array_element_4))
              (Variables|/Game/OTYMI/Blueprint/BP_Rotation_Kitchen_LD1ToLD2.BP_Rotation_Kitchen_LD1ToLD2_C|SetDid%20Turn%20? _asbp_rotation_kitchen_ld1to_ld2 (Variables|/Game/OTYMI/Blueprint/CheckPoint/GI_CheckPoint.GI_CheckPoint_C|GetDid%20Turn%20?K1-2 (Variables|Default|GetAs%20GI%20Check%20Point))))))))
    (Transformation|SetActorLocation (Variables|Default|GetMultipriseRef) (Variables|/Game/OTYMI/Blueprint/CheckPoint/GI_CheckPoint.GI_CheckPoint_C|GetMultiprise%20pose (Variables|Default|GetAs%20GI%20Check%20Point)) false false)
    (Transformation|SetWorldLocation (Variables|/Game/OTYMI/Character/BP_Multiprise.BP_Multiprise_C|GetMultiprise (Variables|Default|GetMultipriseRef)) (Variables|/Game/OTYMI/Blueprint/CheckPoint/GI_CheckPoint.GI_CheckPoint_C|GetMultiprise%20pose (Variables|Default|GetAs%20GI%20Check%20Point)) false false)
    (for _array_element_5 (Variables|Default|GetPlayer%20list)
      (Variables|Default|SetArray%20Element _array_element_5)
      (switch int (Variables|/Game/ThirdPerson/Blueprints/BP_ThirdPersonCharacter.BP_ThirdPersonCharacter_C|GetPlayerID _array_element_5)
        (:0
          (Transformation|SetActorLocation (Variables|Default|GetArray%20Element) (.Location (Utilities|Struct|BreakStru_Player0Data (Variables|/Game/OTYMI/Blueprint/CheckPoint/GI_CheckPoint.GI_CheckPoint_C|GetPlayer%20data0 (Variables|Default|GetAs%20GI%20Check%20Point)))) false false))
        (:1
          (Transformation|SetActorLocation (Variables|Default|GetArray%20Element) (.Location (Utilities|Struct|BreakStru_Player0Data (Variables|/Game/OTYMI/Blueprint/CheckPoint/GI_CheckPoint.GI_CheckPoint_C|GetPlayer%20data1 (Variables|Default|GetAs%20GI%20Check%20Point)))) false false))
        (:2
          (Transformation|SetActorLocation (Variables|Default|GetArray%20Element) (.Location (Utilities|Struct|BreakStru_Player0Data (Variables|/Game/OTYMI/Blueprint/CheckPoint/GI_CheckPoint.GI_CheckPoint_C|GetPlayer%20data2 (Variables|Default|GetAs%20GI%20Check%20Point)))) false false))
        (:3
          (Transformation|SetActorLocation (Variables|Default|GetArray%20Element) (.Location (Utilities|Struct|BreakStru_Player0Data (Variables|/Game/OTYMI/Blueprint/CheckPoint/GI_CheckPoint.GI_CheckPoint_C|GetPlayer%20data3 (Variables|Default|GetAs%20GI%20Check%20Point)))) false false))))
    (Development|PrintString "Done")
    (else
      (for _array_element_6 (Variables|Default|GetPlayer%20list)
        (Default|StartDataREF (.AsGI%20Check%20Point (Utilities|Casting|CastToGI_CheckPoint (Game|GetGameInstance))) (Variables|/Game/ThirdPerson/Blueprints/BP_ThirdPersonCharacter.BP_ThirdPersonCharacter_C|GetPlayerID _array_element_6) (Transformation|GetActorLocation _array_element_6) (Transformation|GetActorLocation (Variables|Default|GetMultipriseRef)) (Variables|Default|GetPivot%20Ref) (Variables|Default|GetCamSpline))))))

(event Collision|EventActorBeginOverlap
  (params (OtherActor :type Actor%20Object%20Reference)))

(event EventTick
  (params (DeltaSeconds :type Float%20%28single-precision%29)))

(fn ConstructionScript)