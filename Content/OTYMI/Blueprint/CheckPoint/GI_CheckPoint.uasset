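; Game instance Blueprint that stores checkpoint state for up to four players, the Multiprise and the level.
; StartDataREF records the initial player and Multiprise positions, pivot rotations and camera spline points.
; CheckpointData, gated on a third-person character trigger, refreshes that data plus the spline move point, "Saved"-tagged actor transforms and Salon/Kitchen rotation flags.
; The file only captures state in variables, with no restore logic.
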(event Custom|StartDataREF
  (params (Plyae%20ID :type Integer) (Player%20pose :type Vector) (multiprise%20pose :type Vector) (Pivot%20Ref :type Array%20of%20Actor%20Object%20References) (CamSpline :type Bp%20Camera%20Spline%20Object%20Reference))
  (bind _cam_spline (Variables|/Game/OTYMI/Blueprint/Bp_CameraSpline.Bp_CameraSpline_C|GetCam%20Spline CamSpline))
  (Variables|Default|SetMultiprise%20pose multiprise%20pose)
  (Variables|Default|SetPlayer%20ID Plyae%20ID)
  (Variables|Default|SetPlayer%20Position Player%20pose)
  (switch int (Variables|Default|GetPlayer%20ID)
    (:0
      (Variables|Default|SetPlayer%20data0 (Utilities|Struct|MakeStru_Player0Data (Variables|Default|GetPlayer%20ID) (Variables|Default|GetPlayer%20Position))))
    (:1
      (Variables|Default|SetPlayer%20data1 (Utilities|Struct|MakeStru_Player0Data (Variables|Default|GetPlayer%20ID) (Variables|Default|GetPlayer%20Position))))
    (:2
      (Variables|Default|SetPlayer%20data2 (Utilities|Struct|MakeStru_Player0Data (Variables|Default|GetPlayer%20ID) (Variables|Default|GetPlayer%20Position))))
    (:3
      (Variables|Default|SetPlayer%20data3 (Utilities|Struct|MakeStru_Player0Data (Variables|Default|GetPlayer%20ID) (Variables|Default|GetPlayer%20Position)))))
  (Utilities|Array|Clear (Variables|Default|GetRotationPivot))
  (for _array_element Pivot%20Ref
    (Utilities|Array|Add (Variables|Default|GetRotationPivot) (Transformation|GetActorRotation _array_element))
    (Utilities|Array|Clear (Variables|Default|GetLocationPointSpline))
    (for _index (range 0 (- (Spline|GetNumberOfSplinePoints _cam_spline) 1))
      (Utilities|Array|Add (Variables|Default|GetLocationPointSpline) (Spline|GetLocationatSplinePoint _cam_spline _index "Local")))))

(event Custom|CheckpointData
  (params (PlayerID :type Integer) (PlayerPosition :type Vector) (MultiprisePosition :type Vector) (PivotData :type Array%20of%20Actor%20Object%20References) (trigering%20object :type Actor%20Object%20Reference) (Spline :type Bp%20Camera%20Spline%20Object%20Reference) (Point%20spline%20move? :type Boolean) (%20Sate%20rotate%20enviro :type Array%20of%20Actor%20Object%20References))
  (bind _cam_spline (Variables|/Game/OTYMI/Blueprint/Bp_CameraSpline.Bp_CameraSpline_C|GetCam%20Spline Spline))
  (if (.bSuccess (Utilities|Casting|CastToBP_ThirdPersonCharacter trigering%20object))
    (Variables|Default|SetPoint%20Spline%20Move? Point%20spline%20move?)
    (Variables|Default|SetMultiprise%20pose MultiprisePosition)
    (Variables|Default|SetPlayer%20ID PlayerID)
    (Variables|Default|SetPlayer%20Position PlayerPosition)
    (switch int (Variables|Default|GetPlayer%20ID)
      (:0
        (Variables|Default|SetPlayer%20data0 (Utilities|Struct|MakeStru_Player0Data (Variables|Default|GetPlayer%20ID) (Variables|Default|GetPlayer%20Position))))
      (:1
        (Variables|Default|SetPlayer%20data1 (Utilities|Struct|MakeStru_Player0Data (Variables|Default|GetPlayer%20ID) (Variables|Default|GetPlayer%20Position))))
      (:2
        (Variables|Default|SetPlayer%20data2 (Utilities|Struct|MakeStru_Player0Data (Variables|Default|GetPlayer%20ID) (Variables|Default|GetPlayer%20Position))))
      (:3
        (Variables|Default|SetPlayer%20data3 (Utilities|Struct|MakeStru_Player0Data (Variables|Default|GetPlayer%20ID) (Variables|Default|GetPlayer%20Position)))))
    (Utilities|Array|Clear (Variables|Default|GetRotationPivot))
    (for _array_element PivotData
      (Utilities|Array|Add (Variables|Default|GetRotationPivot) (Transformation|GetActorRotation _array_element)))
    (Utilities|Array|Clear (Variables|Default|GetLocationPointSpline))
    (for _index (range 0 (- (Spline|GetNumberOfSplinePoints _cam_spline) 1))
      (Utilities|Array|Add (Variables|Default|GetLocationPointSpline) (Spline|GetLocationatSplinePoint _cam_spline _index "Local")))
    (Utilities|Array|Clear (Variables|Default|GetLocation%20Objet%20Saved))
    (bind _outactors (Actor|GetAllActorswithTag "Saved"))
    (for _array_element_2 _outactors
      (Utilities|Array|Add (Variables|Default|GetLocation%20Objet%20Saved) (Transformation|GetActorTransform _array_element_2)))
    (for _array_element_3 %20Sate%20rotate%20enviro
      (bind _asbp_rotation_salon_ld1to_ld2 (Utilities|Casting|CastToBP_Rotation_Salon_LD1ToLD2 _array_element_3)
        (:then
          (Variables|Default|SetDid%20Turn%20?LR1-2 (Variables|/Game/OTYMI/Blueprint/BP_Rotation_Salon_LD1ToLD2.BP_Rotation_Salon_LD1ToLD2_C|GetDid%20Turn%20? _asbp_rotation_salon_ld1to_ld2)))
        (:CastFailed
          (bind _asbp_rotation_salon_ld2to_ld3 (Utilities|Casting|CastToBP_Rotation_Salon_LD2ToLD3 _array_element_3)
            (:then
              (Variables|Default|SetDid%20Turn%20?LR2-3 (Variables|/Game/OTYMI/Blueprint/BP_Rotation_Salon_LD2ToLD3.BP_Rotation_Salon_LD2ToLD3_C|GetDid%20Turn%20? _asbp_rotation_salon_ld2to_ld3)))
            (:CastFailed
              (bind _asbp_rotation_kitchen_ld1to_ld2 (Utilities|Casting|CastToBP_Rotation_Kitchen_LD1ToLD2 _array_element_3))
              (Variables|Default|SetDid%20Turn%20?K1-2 (Variables|/Game/OTYMI/Blueprint/BP_Rotation_Kitchen_LD1ToLD2.BP_Rotation_Kitchen_LD1ToLD2_C|GetDid%20Turn%20? _asbp_rotation_kitchen_ld1to_ld2)))))))
    (Development|PrintString "Saved")))