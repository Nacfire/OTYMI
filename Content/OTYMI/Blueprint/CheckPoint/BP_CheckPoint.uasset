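; Checkpoint trigger volume that saves progress to the GI_CheckPoint game instance, with its box scaled by the construction script.
; Overlaps by player capsules collect unique characters until the required count is reached, while an actor tagged "Mutliprise" triggers the save directly.
; The save passes player ID and position, Multiprise position, pivot, triggering object, camera spline and spline-move data, then flags the checkpoint active.
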(event OnComponentBeginOverlap(Box)
  (params (OverlappedComponent :type Primitive%20Component%20Object%20Reference) (OtherActor :type Actor%20Object%20Reference) (OtherComp :type Primitive%20Component%20Object%20Reference) (OtherBodyIndex :type Integer) (bFromSweep :type Boolean) (SweepResult :type Hit%20Result%20Structure%20%28by%20ref%29))
  (bind _returnvalue (Game|GetGameInstance))
  (bind _asgi_check_point (Utilities|Casting|CastToGI_CheckPoint _returnvalue))
  (if (Components|ComponentHasTag OtherComp "PlayerCapsule")
    (bind _output_get (Variables|Default|SetAs%20BP%20Third%20Person%20Character (.AsBP%20Third%20Person%20Character (Utilities|Casting|CastToBP_ThirdPersonCharacter OtherActor))))
    (Utilities|Array|AddUnique (Variables|Default|GetPlayerPastArray) _output_get)
    (if (== (Utilities|Array|Length (Variables|Default|GetPlayerPastArray)) (Variables|Default|GetPlayer%20need%20to%20Activate))
      (Default|CheckpointData _asgi_check_point (Variables|/Game/ThirdPerson/Blueprints/BP_ThirdPersonCharacter.BP_ThirdPersonCharacter_C|GetPlayerID (Variables|Default|GetAs%20BP%20Third%20Person%20Character)) (Transformation|GetActorLocation (Variables|Default|GetAs%20BP%20Third%20Person%20Character)) (Transformation|GetWorldLocation (Variables|/Game/OTYMI/Character/BP_Multiprise.BP_Multiprise_C|GetMultiprise (Variables|Default|GetMultiprise))) (Variables|Default|GetPivot) OtherActor (Variables|Default|GetCamSpine) (Variables|/Game/OTYMI/Blueprint/BP_MovePointOnCameraSpline.BP_MovePointOnCameraSpline_C|GetActivate (Variables|Default|Getmove%20point%20spline)) :!label _label)
      (Variables|/Game/OTYMI/Blueprint/CheckPoint/GI_CheckPoint.GI_CheckPoint_C|SetbIsCheckPointActive _asgi_check_point true))
    (elif (Actor|ActorHasTag OtherActor "Mutliprise")
      (goto _label))))

(event EventBeginPlay)

(event Collision|EventActorBeginOverlap
  (params (OtherActor :type Actor%20Object%20Reference)))

(event EventTick
  (params (DeltaSeconds :type Float%20%28single-precision%29)))

(fn ConstructionScript
  (Transformation|SetWorldScale3D (Variables|Default|GetBox) (Variables|Default|GetScale)))