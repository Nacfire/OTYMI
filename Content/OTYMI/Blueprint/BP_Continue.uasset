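; BP_Continue is an actor that restores player positions from a saved checkpoint when play begins.
; It finds BP_ConditionDefaite in the level and reads the GI_CheckPoint game instance, proceeding only if a checkpoint is active.
; For each entry in the defeat-condition actor's PlayerList, it uses PlayerID to move the game instance's PlayerListDATA actor to its stored PlayerPose, without sweep or teleport.
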(event EventBeginPlay
  (bind _returnvalue (Actor|GetActorOfClass "/Game/OTYMI/Blueprint/BP_ConditionDefaite.BP_ConditionDefaite_C"))
  (Variables|Default|SetBP_ConditionDefaite _returnvalue)
  (bind _asgi_check_point (Utilities|Casting|CastToGI_CheckPoint (Game|GetGameInstance)))
  (Variables|Default|SetAs%20GI%20Check%20Point _asgi_check_point)
  (if (Variables|/Game/OTYMI/Blueprint/GI_CheckPoint.GI_CheckPoint_C|GetbIsCheckPointActive _asgi_check_point)
    (for _array_element (Variables|/Game/OTYMI/Blueprint/BP_ConditionDefaite.BP_ConditionDefaite_C|GetPlayerList (Variables|Default|GetBP_ConditionDefaite))
      (Transformation|SetActorLocation (Utilities|Array|Get(acopy) (Variables|/Game/OTYMI/Blueprint/GI_CheckPoint.GI_CheckPoint_C|GetPlayerListDATA (Variables|Default|GetAs%20GI%20Check%20Point)) (Variables|/Game/ThirdPerson/Blueprints/BP_ThirdPersonCharacter.BP_ThirdPersonCharacter_C|GetPlayerID _array_element)) (Utilities|Array|Get(acopy) (Variables|/Game/OTYMI/Blueprint/GI_CheckPoint.GI_CheckPoint_C|GetPlayer%20pose (Variables|Default|GetAs%20GI%20Check%20Point)) (Variables|/Game/ThirdPerson/Blueprints/BP_ThirdPersonCharacter.BP_ThirdPersonCharacter_C|GetPlayerID _array_element)) false false))))

(event Collision|EventActorBeginOverlap
  (params (OtherActor :type Actor%20Object%20Reference)))

(event EventTick
  (params (DeltaSeconds :type Float%20%28single-precision%29)))

(fn ConstructionScript)