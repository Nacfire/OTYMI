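; One-shot trigger actor that rotates a referenced pivot, apparently for the Salon LD2-to-LD3 transition.
; The box trigger counts third-person characters through their capsule overlaps, checking on each entry whether the required player count is reached.
; When it is, a timeline smoothly drives the pivot mesh's world yaw, and a flag prevents repeats.
; Disconnected leftover logic covers a screen fade and WIP Multiprise axis-constraint swapping.
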(event OnComponentBeginOverlap(RotationBoxTrigger)
  (params (OverlappedComponent :type Primitive%20Component%20Object%20Reference) (OtherActor :type Actor%20Object%20Reference) (OtherComp :type Primitive%20Component%20Object%20Reference) (OtherBodyIndex :type Integer) (bFromSweep :type Boolean) (SweepResult :type Hit%20Result%20Structure%20%28by%20ref%29))
  ;[0.15 0.15 0.15 0.5] Update Player count on Begin Overlap
  (bind _asbp_third_person_character (Utilities|Casting|CastToBP_ThirdPersonCharacter OtherActor))
  (if (== (Variables|/Script/Engine.Character|GetCapsuleComponent _asbp_third_person_character) OtherComp)
    (Variables|Default|SetNumberOfPlayer (+ (Variables|Default|GetNumberOfPlayer) 1))
    (CallFunction|CheckPlayerCount)))

(event OnComponentEndOverlap(RotationBoxTrigger)
  (params (OverlappedComponent :type Primitive%20Component%20Object%20Reference) (OtherActor :type Actor%20Object%20Reference) (OtherComp :type Primitive%20Component%20Object%20Reference) (OtherBodyIndex :type Integer))
  ;[0.15 0.15 0.15 0.5] Update Player count on End Overlap
  (bind _asbp_third_person_character (Utilities|Casting|CastToBP_ThirdPersonCharacter OtherActor))
  (if (== (Variables|/Script/Engine.Character|GetCapsuleComponent _asbp_third_person_character) OtherComp)
    (Variables|Default|SetNumberOfPlayer (- (Variables|Default|GetNumberOfPlayer) 1))
    (if (<= (Variables|Default|GetNumberOfPlayer) 0)
      (Variables|Default|SetNumberOfPlayer 0))))

(event Custom|CheckPlayerCount
  (if (not (Variables|Default|GetDid%20Turn%20?))
    (if (== (Variables|Default|GetNumberOfPlayer) (Variables|Default|GetPlayer%20To%20Rotate))
      (Variables|Default|SetDid%20Turn%20? true)
      (bind _rot_z (Timeline|Smooth%20Pivot%20Rot PlayFromStart)
        (:Update
          (Transformation|SetWorldRotation (Variables|/Script/Engine.StaticMeshActor|GetStaticMeshComponent (Variables|Default|GetPivot%20Ref)) (Math|Rotator|MakeRotator 0.0 0.0 _rot_z) false false))))))

(event EventBeginPlay
  (Input|EnableInput 0))

(fn ConstructionScript)