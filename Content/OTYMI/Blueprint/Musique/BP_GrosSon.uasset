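; BP_GrosSon is a music player Blueprint with an Audio component that starts its default Sound on BeginPlay.
; A custom event takes a GenreChépaSon key, stops playback, looks up the matching sound in the SonLibrairie map and plays it from the start.
; The switch is immediate, with no fade and no check that the key was found.
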(event Custom|CustomEvent
  (params (GenreChépaSon :type String))
  (bind _audio (Variables|Default|GetAudio))
  (Audio|Components|Audio|Stop _audio)
  (Audio|Components|Audio|SetSound _audio (.Value (Utilities|Map|Find (Variables|Default|GetSonLibrairie) GenreChépaSon)))
  (Audio|Components|Audio|Play (Variables|Default|GetAudio) 0.0))

(event Collision|EventActorBeginOverlap
  (params (OtherActor :type Actor%20Object%20Reference)))

(event EventTick
  (params (DeltaSeconds :type Float%20%28single-precision%29)))

(event EventBeginPlay
  (bind _audio (Variables|Default|GetAudio))
  (Audio|Components|Audio|SetSound _audio (Variables|Default|GetSound))
  (Audio|Components|Audio|Play _audio 0.0))

(fn ConstructionScript)