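; BP_ConditionDefaite is a defeat-condition actor that returns the game to the main menu when every player is disconnected.
; A looping timer started on BeginPlay polls every tenth of a second, counting PlayerList entries flagged IsPlayerDeconnected.
; When the count equals the list length, it opens the MainMenu level, which also happens if the list is empty.
; PlayerList is not filled within this Blueprint.
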(event Custom|Timer
  (Variables|Default|SetConteurDisconect 0)
  (for _array_element (Variables|Default|GetPlayerList)
    (if (Variables|/Game/ThirdPerson/Blueprints/BP_ThirdPersonCharacter.BP_ThirdPersonCharacter_C|GetIsPlayerDeconnected _array_element)
      (Variables|Default|SetConteurDisconect (+ (Variables|Default|GetConteurDisconect) 1))))
  (if (== (Variables|Default|GetConteurDisconect) (Utilities|Array|Length (Variables|Default|GetPlayerList)))
    (Game|OpenLevel(byObjectReference) "/Game/OTYMI/UI/MainMenu/MainMenu.MainMenu")))

(event EventBeginPlay
  (Utilities|Time|SetTimerbyEvent (delegate Custom|Timer) 0.1 true))

(event Collision|EventActorBeginOverlap
  (params (OtherActor :type Actor%20Object%20Reference)))

(event EventTick
  (params (DeltaSeconds :type Float%20%28single-precision%29)))

(fn ConstructionScript)