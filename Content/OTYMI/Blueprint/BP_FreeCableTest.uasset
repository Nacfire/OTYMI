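; BP_FreeCableTest is a test cable actor that makes a rope spline follow a chain of twenty capsule components.
; BeginPlay gathers the capsules into an array, and Tick moves each spline point to its capsule's world location, passed as Local space.
; The construction script does the same in World space, then adds a spline mesh component per segment without setting its shape or updating it later.
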(event EventBeginPlay
  (Utilities|Array|Add (Variables|Default|GetCapsules) (Variables|Default|GetCapsule_01))
  (Utilities|Array|Add (Variables|Default|GetCapsules) (Variables|Default|GetCapsule_02))
  (Utilities|Array|Add (Variables|Default|GetCapsules) (Variables|Default|GetCapsule_03))
  (Utilities|Array|Add (Variables|Default|GetCapsules) (Variables|Default|GetCapsule_04))
  (Utilities|Array|Add (Variables|Default|GetCapsules) (Variables|Default|GetCapsule_05))
  (Utilities|Array|Add (Variables|Default|GetCapsules) (Variables|Default|GetCapsule_06))
  (Utilities|Array|Add (Variables|Default|GetCapsules) (Variables|Default|GetCapsule_07))
  (Utilities|Array|Add (Variables|Default|GetCapsules) (Variables|Default|GetCapsule_08))
  (Utilities|Array|Add (Variables|Default|GetCapsules) (Variables|Default|GetCapsule_09))
  (Utilities|Array|Add (Variables|Default|GetCapsules) (Variables|Default|GetCapsule_010))
  (Utilities|Array|Add (Variables|Default|GetCapsules) (Variables|Default|GetCapsule_011))
  (Utilities|Array|Add (Variables|Default|GetCapsules) (Variables|Default|GetCapsule_012))
  (Utilities|Array|Add (Variables|Default|GetCapsules) (Variables|Default|GetCapsule_013))
  (Utilities|Array|Add (Variables|Default|GetCapsules) (Variables|Default|GetCapsule_014))
  (Utilities|Array|Add (Variables|Default|GetCapsules) (Variables|Default|GetCapsule_015))
  (Utilities|Array|Add (Variables|Default|GetCapsules) (Variables|Default|GetCapsule_016))
  (Utilities|Array|Add (Variables|Default|GetCapsules) (Variables|Default|GetCapsule_017))
  (Utilities|Array|Add (Variables|Default|GetCapsules) (Variables|Default|GetCapsule_018))
  (Utilities|Array|Add (Variables|Default|GetCapsules) (Variables|Default|GetCapsule_019))
  (Utilities|Array|Add (Variables|Default|GetCapsules) (Variables|Default|GetCapsule_020)))

(event EventTick
  (params (DeltaSeconds :type Float%20%28single-precision%29))
  (for _index (range 0 (- (Variables|Default|GetNumberOfCapsule) 1))
    (Spline|SetLocationatSplinePoint (Variables|Default|GetRopeSpline) _index (Transformation|GetWorldLocation (Utilities|Array|Get(acopy) (Variables|Default|GetCapsules) _index)) "Local" true)))

(fn ConstructionScript
  (for _index (range 0 (- (Variables|Default|GetNumberOfCapsule) 1))
    (Spline|SetLocationatSplinePoint (Variables|Default|GetRopeSpline) _index (Transformation|GetWorldLocation (Utilities|Array|Get(acopy) (Variables|Default|GetCapsules) _index)) "World" true))
  (for _index_2 (range 0 (- (Variables|Default|GetNumberOfCapsule) 2))
    (bind _returnvalue (AddComponent|AddSplineMeshComponent false))
    (Variables|Default|SetSm_i _returnvalue)))