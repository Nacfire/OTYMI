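; Test Blueprint that builds a cable chain of instanced link meshes along local X in the Construction Script.
; A loop steps by a spacing and uses a FlipFlop to rotate every other HISM link 90 degrees.
; Each link also gets an offset physics constraint component, but no components are passed to constrain.
; An uncalled spline helper has zeroed inputs, and the mesh-length calculation never runs.
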(event EventBeginPlay)

(event Collision|EventActorBeginOverlap
  (params (OtherActor :type Actor%20Object%20Reference)))

(event EventTick
  (params (DeltaSeconds :type Float%20%28single-precision%29)))

(fn ConstructionScript
  (Components|StaticMesh|SetStaticMesh (Variables|Default|GetHISM_Chain) (Variables|Default|GetChain_SM))
  (for _index (range 0 (- (Variables|Default|GetChainNumber) 1))
    (Variables|Default|SetNewChainPos (+ (Variables|Default|GetNewChainPos) (Variables|Default|GetSpacing)))
    (Utilities|FlowControl|FlipFlop
      (:A
        (Variables|Default|SetRotateChain false)
        (Components|InstancedStaticMesh|AddInstance (Variables|Default|GetHISM_Chain) (Math|Transform|MakeTransform (Math|Vector|MakeVector (Variables|Default|GetNewChainPos) 0.0 0.0) "0, 0, 0" "0.100000,0.100000,0.100000") false))
      (:B
        (Variables|Default|SetRotateChain true)
        (Components|InstancedStaticMesh|AddInstance (Variables|Default|GetHISM_Chain) (Math|Transform|MakeTransform (Math|Vector|MakeVector (Variables|Default|GetNewChainPos) 0.0 0.0) "0.000000,0.000000,90.000000" "0.100000,0.100000,0.100000") false)))
    (bind _returnvalue (AddComponent|AddPhysicsConstraintComponent false (Math|Transform|MakeTransform (Math|Vector|MakeVector (+ (Variables|Default|GetNewChainPos) 1e+01) 0.0 0.0) "0, 0, 0" "0.500000,0.500000,0.500000")))
    (if (Variables|Default|GetRotateChain)
      (Class|PhysicsConstraintComponent|SetConstrainedComponents _returnvalue 0 "None" 0 "None"))))

(fn GetLocationandTangent
  (params (A :type Integer))
  (bind _spline (Variables|Default|GetSpline))
  (return (Spline|GetLocationatDistanceAlongSpline _spline (* A 0.0) "Local") (Math|Vector|ClampVectorSize (Spline|GetTangentatDistanceAlongSpline _spline 0.0 "Local") 0.0 0.0)))