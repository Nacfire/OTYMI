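; Physics-simulated hanging chain actor that spawns a row of link meshes along X, alternately rotated, with the first link pinned.
; BeginPlay joins neighbouring links with angle-limited physics constraints at hard-coded 20-unit spacing; the construction script can optionally build the same chain.
; A spline gets one point per link and follows them on Tick.
; Spline mesh skinning is unfinished: its positioning code is disconnected.
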(event EventBeginPlay
  (bind _mesh_scale (Variables|Default|GetMesh%20Scale))
  (bind _linksarray (Variables|Default|GetLinksArray))
  ;[0.15 0.15 0.15 0.5] Set Static Mesh (Chains)
  (Variables|Default|SetBase%20Location (+ (Variables|Default|GetStartOffset) (Transformation|GetActorLocation)))
  (Variables|Default|SetBase%20Forward (Transformation|GetActorForwardVector))
  (Utilities|Array|Clear (Variables|Default|GetLinksArray))
  (for _index (range 0 (- (Variables|Default|GetNbLinks) 1))
    (Variables|Default|SetBeginPlay%20Links%20Index _index)
    (Utilities|FlowControl|FlipFlop
      (:A
        (Variables|Default|SetRotateChain false))
      (:B
        (Variables|Default|SetRotateChain true)))
    (bind _returnvalue (AddComponent|AddStaticMeshComponent false))
    (Components|StaticMesh|SetStaticMesh _returnvalue (Variables|Default|GetLinks_SM))
    (if (== (Variables|Default|GetBeginPlay%20Links%20Index) 0)
      (Physics|SetSimulatePhysics _returnvalue false)
      (else
        (Physics|SetSimulatePhysics _returnvalue true)))
    (Collision|SetCollisionEnabled _returnvalue "QueryAndPhysics")
    (if (Variables|Default|GetRotateChain)
      (Transformation|SetWorldTransform _returnvalue (Math|Transform|MakeTransform (Math|Vector|MakeVector (+ (.x (Variables|Default|GetBase%20Location)) (* (Variables|Default|GetLinks%20Spacing) (Variables|Default|GetBeginPlay%20Links%20Index))) (.y (Variables|Default|GetBase%20Location)) (.z (Variables|Default|GetBase%20Location))) "0.000000,0.000000,90.000000" _mesh_scale) false false)
      (else
        (Transformation|SetWorldTransform _returnvalue (Math|Transform|MakeTransform (Math|Vector|MakeVector (+ (.x (Variables|Default|GetBase%20Location)) (* (Variables|Default|GetLinks%20Spacing) (Variables|Default|GetBeginPlay%20Links%20Index))) (.y (Variables|Default|GetBase%20Location)) (.z (Variables|Default|GetBase%20Location))) "0, 0, 0" _mesh_scale) false false)))
    (Utilities|Array|Add (Variables|Default|GetLinksArray) _returnvalue))
  ;[0.15 0.15 0.15 0.5] Set Physics Constraints
  (Utilities|Array|Clear (Variables|Default|GetPhysicsConstraintsArray))
  (for _index_2 (range 0 (- (Variables|Default|GetNbLinks) 2))
    (Variables|Default|SetBeginPlay%20Physics%20Constraint%20Index _index_2)
    (bind _returnvalue_2 (AddComponent|AddPhysicsConstraintComponent false (Math|Transform|MakeTransform "10.000000,0.000000,0.000000" "0, 0, 0" "1.000000,1.000000,1.000000")))
    (Transformation|SetWorldTransform _returnvalue_2 (Math|Transform|MakeTransform (Math|Vector|MakeVector (+ (.x (Variables|Default|GetBase%20Location)) (* (Variables|Default|GetBeginPlay%20Physics%20Constraint%20Index) 20)) (.y (Variables|Default|GetBase%20Location)) (.z (Variables|Default|GetBase%20Location))) "0, 0, 0" "1.000000,1.000000,1.000000") false false)
    (Class|PhysicsConstraintComponent|SetConstrainedComponents _returnvalue_2 (Utilities|Array|Get(acopy) _linksarray (Variables|Default|GetBeginPlay%20Physics%20Constraint%20Index)) "None" (Utilities|Array|Get(acopy) _linksarray (+ (Variables|Default|GetBeginPlay%20Physics%20Constraint%20Index) 1)) "None")
    (Class|PhysicsConstraintComponent|SetAngularSwing1Limit _returnvalue_2 "ACM_Limited" (Variables|Default|GetConstraints%20Angular%20Swing%20Limit))
    (Class|PhysicsConstraintComponent|SetAngularSwing2Limit _returnvalue_2 "ACM_Limited" (Variables|Default|GetConstraints%20Angular%20Swing%20Limit))
    (Class|PhysicsConstraintComponent|SetAngularTwistLimit _returnvalue_2 "ACM_Limited" (Variables|Default|GetConstraint%20Angular%20Twist%20limit))
    (Class|PhysicsConstraintComponent|SetDisableCollision _returnvalue_2 true)
    (Utilities|Array|Add (Variables|Default|GetPhysicsConstraintsArray) _returnvalue_2))
  ;[0.15 0.15 0.15 0.5] Set Spline Points
  (Spline|ClearSplinePoints (Variables|Default|GetSpline) true)
  (for _index_3 (range 0 (- (Variables|Default|GetNbLinks) 1))
    (Spline|AddSplinePoint (Variables|Default|GetSpline) (Variables|/Script/Engine.SceneComponent|GetRelativeLocation (Utilities|Array|Get(acopy) (Variables|Default|GetLinksArray) _index_3)) "Local" true)))

(event EventTick
  (params (DeltaSeconds :type Float%20%28single-precision%29))
  ;[0.15 0.15 0.15 0.5] Update Spline Points Location
  (for _index (range 0 (- (Variables|Default|GetNbLinks) 1))
    (Variables|Default|SetTick%20Spline%20Points%20Index _index)
    (Variables|Default|SetSplinePointLoc (Variables|/Script/Engine.SceneComponent|GetRelativeLocation (Utilities|Array|Get(acopy) (Variables|Default|GetLinksArray) (Variables|Default|GetTick%20Spline%20Points%20Index))))
    (Spline|SetLocationatSplinePoint (Variables|Default|GetSpline) (Variables|Default|GetTick%20Spline%20Points%20Index) (Variables|Default|GetSplinePointLoc) "Local" true)))

(fn ConstructionScript
  (bind _mesh_scale (Variables|Default|GetMesh%20Scale))
  (bind _linksarray (Variables|Default|GetLinksArray))
  ;[0.15 0.15 0.15 0.5] Set Static Mesh (Chains)
  (Variables|Default|SetBase%20Location (+ (Variables|Default|GetStartOffset) (Transformation|GetActorLocation)))
  (Variables|Default|SetBase%20Forward (Transformation|GetActorForwardVector))
  (if (Variables|Default|GetActivate%20Construction%20Script)
    (Utilities|Array|Clear (Variables|Default|GetLinksArray))
    (for _index (range 0 (- (Variables|Default|GetNbLinks) 1))
      (Variables|Default|SetBeginPlay%20Links%20Index _index)
      (Utilities|FlowControl|FlipFlop
        (:A
          (Variables|Default|SetRotateChain false))
        (:B
          (Variables|Default|SetRotateChain true)))
      (bind _returnvalue (AddComponent|AddStaticMeshComponent false))
      (Components|StaticMesh|SetStaticMesh _returnvalue (Variables|Default|GetLinks_SM))
      (if (== (Variables|Default|GetBeginPlay%20Links%20Index) 0)
        (Physics|SetSimulatePhysics _returnvalue false)
        (else
          (Physics|SetSimulatePhysics _returnvalue true)))
      (Collision|SetCollisionEnabled _returnvalue "QueryAndPhysics")
      (if (Variables|Default|GetRotateChain)
        (Transformation|SetWorldTransform _returnvalue (Math|Transform|MakeTransform (Math|Vector|MakeVector (* (Variables|Default|GetLinks%20Spacing) (Variables|Default|GetBeginPlay%20Links%20Index)) 0.0 0.0) "0.000000,0.000000,90.000000" _mesh_scale) false false)
        (else
          (Transformation|SetWorldTransform _returnvalue (Math|Transform|MakeTransform (Math|Vector|MakeVector (* (Variables|Default|GetLinks%20Spacing) (Variables|Default|GetBeginPlay%20Links%20Index)) 0.0 0.0) "0, 0, 0" _mesh_scale) false false)))
      (Class|PrimitiveComponent|SetUseCCD _returnvalue true "None")
      (Utilities|Array|Add (Variables|Default|GetLinksArray) _returnvalue))
    ;[0.15 0.15 0.15 0.5] Set Physics Constraints
    (Utilities|Array|Clear (Variables|Default|GetPhysicsConstraintsArray))
    (for _index_2 (range 0 (- (Variables|Default|GetNbLinks) 2))
      (Variables|Default|SetBeginPlay%20Physics%20Constraint%20Index _index_2)
      (bind _returnvalue_2 (AddComponent|AddPhysicsConstraintComponent false (Math|Transform|MakeTransform "10.000000,0.000000,0.000000" "0, 0, 0" "1.000000,1.000000,1.000000")))
      (Transformation|SetWorldTransform _returnvalue_2 (Math|Transform|MakeTransform (Math|Vector|MakeVector (* (Variables|Default|GetBeginPlay%20Physics%20Constraint%20Index) 20) 0.0 0.0) "0, 0, 0" "1.000000,1.000000,1.000000") false false)
      (Class|PhysicsConstraintComponent|SetConstrainedComponents _returnvalue_2 (Utilities|Array|Get(acopy) _linksarray (Variables|Default|GetBeginPlay%20Physics%20Constraint%20Index)) "None" (Utilities|Array|Get(acopy) _linksarray (+ (Variables|Default|GetBeginPlay%20Physics%20Constraint%20Index) 1)) "None")
      (Class|PhysicsConstraintComponent|SetAngularSwing1Limit _returnvalue_2 "ACM_Limited" (Variables|Default|GetConstraints%20Angular%20Swing%20Limit))
      (Class|PhysicsConstraintComponent|SetAngularSwing2Limit _returnvalue_2 "ACM_Limited" (Variables|Default|GetConstraints%20Angular%20Swing%20Limit))
      (Class|PhysicsConstraintComponent|SetAngularTwistLimit _returnvalue_2 "ACM_Limited" (Variables|Default|GetConstraint%20Angular%20Twist%20limit))
      (Class|PhysicsConstraintComponent|SetDisableCollision _returnvalue_2 true)
      (Utilities|Array|Add (Variables|Default|GetPhysicsConstraintsArray) _returnvalue_2))
    ;[0.15 0.15 0.15 0.5] Set Spline Points
    (Spline|ClearSplinePoints (Variables|Default|GetSpline) true)
    (for _index_3 (range 0 (- (Variables|Default|GetNbLinks) 1))
      (Spline|AddSplinePoint (Variables|Default|GetSpline) (Variables|/Script/Engine.SceneComponent|GetRelativeLocation (Utilities|Array|Get(acopy) (Variables|Default|GetLinksArray) _index_3)) "Local" true))
    ;[0.15 0.15 0.15 0.5] Set Spline Mesh
    (Utilities|Array|Clear (Variables|Default|GetSplineMeshArray))
    (for _index_4 (range 0 (- (Variables|Default|GetNbLinks) 2))
      (bind _returnvalue_3 (AddComponent|AddSplineMeshComponent false))
      (Components|StaticMesh|SetStaticMesh _returnvalue_3 (Variables|Default|GetSplineMeshVisual))
      (Collision|SetCollisionEnabled _returnvalue_3 "NoCollision")
      (Transformation|SetMobility _returnvalue_3 "Movable")
      (Utilities|Array|Add (Variables|Default|GetSplineMeshArray) _returnvalue_3))))

(fn GetLocationandTangent
  (params (Index :type Integer))
  (bind _spline (Variables|Default|GetSpline))
  (bind _sm_cylinder_length (Variables|Default|GetSM_Cylinder_Length))
  (bind _returnvalue (* Index _sm_cylinder_length))
  (return (Spline|GetLocationatDistanceAlongSpline _spline _returnvalue "Local") (Math|Vector|ClampVectorSize (Spline|GetTangentatDistanceAlongSpline _spline _returnvalue "Local") 0.0 (Variables|Default|GetSM_Cylinder_Length))))