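; Test spline actor in the Cable folder that lays a static mesh along its spline in the construction script.
; SpacesMesh places half-scale copies at spaced intervals; otherwise spline mesh segments, sized by the mesh's forward-axis bounds, join end to end.
; GetLocationAndTangent supplies segment ends, always sampling the tangent at distance zero.
; Segment up direction blends UpVectors entries or falls back to the spline's, with optional ShowUp debug arrows.
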(event EventBeginPlay)

(event Collision|EventActorBeginOverlap
  (params (OtherActor :type Actor%20Object%20Reference)))

(event EventTick
  (params (DeltaSeconds :type Float%20%28single-precision%29)))

(fn ConstructionScript
  (bind _spline (Variables|Default|GetSpline))
  (bind _spline_2 (Variables|Default|GetSpline))
  (bind _splinemesh (Variables|Default|GetSplineMesh))
  (bind _spline_3 (Variables|Default|GetSpline))
  (bind _returnvalue (Spline|GetSplineLength _spline_2))
  (bind _returnvalue_2 (StaticMesh|GetBoundingBox _splinemesh))
  (bind _returnvalue_3 (- (.max _returnvalue_2) (.min _returnvalue_2)))
  (if (Utilities|Enum|Equal(Enum) (Variables|Default|GetIn%20Forward%20Axis) "X")
    (Variables|Default|SetMesh%20Length (.x _returnvalue_3))
    (elif (Utilities|Enum|Equal(Enum) (Variables|Default|GetIn%20Forward%20Axis) "Y")
      (Variables|Default|SetMesh%20Length (.y _returnvalue_3))
      (else
        (Variables|Default|SetMesh%20Length (.z _returnvalue_3)))))
  (if (Variables|Default|GetSpaces%20Mesh)
    (Variables|Default|SetSegment%20Length (+ (Variables|Default|GetSpacing) (Variables|Default|GetMesh%20Length)))
    (for _index (range 0 (Math|Float|Truncate (/ (Spline|GetSplineLength (Variables|Default|GetSpline)) (Variables|Default|GetSegment%20Length))))
      (Variables|Default|SetIndex _index)
      (bind _returnvalue_4 (AddComponent|AddSplineMeshComponent false (Math|Transform|MakeTransform (Spline|GetLocationatDistanceAlongSpline _spline (* (Variables|Default|GetIndex) (Variables|Default|GetSegment%20Length)) "Local") (Math|Rotator|CombineRotators (Variables|Default|GetMeshRotation) (Spline|GetRotationatDistanceAlongSpline _spline (* (Variables|Default|GetIndex) (Variables|Default|GetSegment%20Length)) "Local")) "0.500000,0.500000,0.500000")))
      (Components|StaticMesh|SetStaticMesh _returnvalue_4 (Variables|Default|GetSplineMesh))
      (Collision|SetCollisionEnabled _returnvalue_4 "QueryAndPhysics")
      (SplineMesh|SetForwardAxis _returnvalue_4 (Variables|Default|GetIn%20Forward%20Axis) true))
    (else
      (for _index_2 (range 0 (Math|Float|Truncate (/ (Spline|GetSplineLength (Variables|Default|GetSpline)) (Variables|Default|GetMesh%20Length))))
        (Variables|Default|SetIndex _index_2)
        (bind _returnvalue_5 (AddComponent|AddSplineMeshComponent false))
        (Components|StaticMesh|SetStaticMesh _returnvalue_5 (Variables|Default|GetSplineMesh))
        (Collision|SetCollisionEnabled _returnvalue_5 "QueryAndPhysics")
        (SplineMesh|SetForwardAxis _returnvalue_5 (Variables|Default|GetIn%20Forward%20Axis) true)
        (bind (_location _tangent) (CallFunction|GetLocationandTangent (Variables|Default|GetIndex)))
        (bind (_location_2 _tangent_2) (CallFunction|GetLocationandTangent (+ (Variables|Default|GetIndex) 1)))
        (SplineMesh|SetStartandEnd _returnvalue_5 _location _tangent _location_2 _tangent_2 true :!class /Script/Engine.SplineMeshComponent)
        (Variables|Default|SetInput%20Key (Class|SplineComponent|GetInputKeyValueatDistanceAlongSpline (Variables|Default|GetSpline) (+ (+ (* (Variables|Default|GetIndex) (Variables|Default|GetMesh%20Length)) (Math|Float|SelectFloat (+ (* (Variables|Default|GetIndex) (Variables|Default|GetMesh%20Length)) (Variables|Default|GetMesh%20Length)) _returnvalue (< (+ (* (Variables|Default|GetIndex) (Variables|Default|GetMesh%20Length)) (Variables|Default|GetMesh%20Length)) _returnvalue))) 2.0)))
        (if (and (.ReturnValue (Utilities|Map|Find (Variables|Default|GetUp%20Vectors) (Math|Float|Ceil (Variables|Default|GetInput%20Key)))) (.ReturnValue (Utilities|Map|Find (Variables|Default|GetUp%20Vectors) (Math|Float|Floor (Variables|Default|GetInput%20Key)))))
          (SplineMesh|SetSplineUpDir _returnvalue_5 (Math|Vector|Lerp(Vector) (.Value (Utilities|Map|Find (Variables|Default|GetUp%20Vectors) (Math|Float|Ceil (Variables|Default|GetInput%20Key)))) (.Value (Utilities|Map|Find (Variables|Default|GetUp%20Vectors) (Math|Float|Floor (Variables|Default|GetInput%20Key)))) (Math|Float|Fraction (Variables|Default|GetInput%20Key))) true)
          (else
            (SplineMesh|SetSplineUpDir _returnvalue_5 (Class|SplineComponent|GetUpVectoratDistanceAlongSpline (Variables|Default|GetSpline) (+ (/ (- (Math|Float|SelectFloat (+ (* (Variables|Default|GetIndex) (Variables|Default|GetMesh%20Length)) (Variables|Default|GetMesh%20Length)) _returnvalue (< (+ (* (Variables|Default|GetIndex) (Variables|Default|GetMesh%20Length)) (Variables|Default|GetMesh%20Length)) _returnvalue)) (* (Variables|Default|GetIndex) (Variables|Default|GetMesh%20Length))) 2.0) (Math|Float|SelectFloat (+ (* (Variables|Default|GetIndex) (Variables|Default|GetMesh%20Length)) (Variables|Default|GetMesh%20Length)) _returnvalue (< (+ (* (Variables|Default|GetIndex) (Variables|Default|GetMesh%20Length)) (Variables|Default|GetMesh%20Length)) _returnvalue))) "Local") true)))
        (if (Variables|Default|GetShow%20Up)
          (AddComponent|AddArrowComponent false (Math|Transform|MakeTransform (Spline|GetLocationatSplinePoint _spline_3 (Variables|Default|GetIndex) "Local") (Math|Rotator|CombineRotators "90.000000,0.000000,0.000000" (Spline|GetRotationatSplinePoint _spline_3 (Variables|Default|GetIndex) "Local")) "1.000000,5.000000,5.000000")))))))

(fn GetLocationandTangent
  (params (A :type Integer))
  (bind _spline (Variables|Default|GetSpline))
  (return (Spline|GetLocationatDistanceAlongSpline _spline (* A (Variables|Default|GetMesh%20Length)) "Local") (Math|Vector|ClampVectorSize (Spline|GetTangentatDistanceAlongSpline _spline 0.0 "Local") 0.0 (Variables|Default|GetMesh%20Length))))