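; BP_Buton is a trigger button that turns on physics simulation for the mesh of a referenced Interactible actor.
; On trigger overlap it compares the actor's class against a BP_ThirdPersonCharacter reference, printing "Not player" on a mismatch.
; The construction script sets the button mesh and scales the button and trigger from variables.
; The DestoyAferGetPhysique branch is empty, and the delayed VFX print and destroy chain is disconnected.
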(event OnComponentBeginOverlap(Trigger)
  (params (OverlappedComponent :type Primitive%20Component%20Object%20Reference) (OtherActor :type Actor%20Object%20Reference) (OtherComp :type Primitive%20Component%20Object%20Reference) (OtherBodyIndex :type Integer) (bFromSweep :type Boolean) (SweepResult :type Hit%20Result%20Structure%20%28by%20ref%29))
  (bind _asactor (Utilities|Casting|CastToActorClass "/Game/ThirdPerson/Blueprints/BP_ThirdPersonCharacter.BP_ThirdPersonCharacter_C"))
  (if (== (Utilities|GetClass OtherActor) _asactor)
    (Physics|SetSimulatePhysics (Variables|/Game/OTYMI/Blueprint/BP_Drop-Object.BP_Drop-Object_C|GetMesh (Variables|Default|GetInteractible)) true)
    (if (Variables|Default|GetDestoy%20afer%20Get%20physique)
      _)
    (else
      (Development|PrintString "Not player" true true "(R=1.000000,G=0.014456,B=0.000000,A=1.000000)"))))

(event EventBeginPlay)

(event Collision|EventActorBeginOverlap
  (params (OtherActor :type Actor%20Object%20Reference)))

(event EventTick
  (params (DeltaSeconds :type Float%20%28single-precision%29)))

(fn ConstructionScript
  (Components|StaticMesh|SetStaticMesh (Variables|Default|GetSM_Buton) (Variables|Default|GetSM_visuel))
  (Transformation|SetWorldScale3D (Variables|Default|GetTrigger) (Variables|Default|GetScaleTriger))
  (Transformation|SetWorldScale3D (Variables|Default|GetSM_Buton) (Variables|Default|GetScaleButon)))