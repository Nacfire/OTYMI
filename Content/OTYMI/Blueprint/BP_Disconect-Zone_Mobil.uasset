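; A moving disconnect hazard zone: overlapping a player capsule disconnects that BP_ThirdPersonCharacter once, guarded by its IsPlayerDeconnected flag.
; The actor slides between its start location and a TargetLocation actor's position via open and close timelines with configurable delays and rates.
; Open and Close trigger movement based on the IsOpen state, and Loop chains the two into continuous back-and-forth motion.
; The construction script sizes the DeathZone from ScaleDeathZone.
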(event OnComponentBeginOverlap(Death-Zone)
  (params (OverlappedComponent :type Primitive%20Component%20Object%20Reference) (OtherActor :type Actor%20Object%20Reference) (OtherComp :type Primitive%20Component%20Object%20Reference) (OtherBodyIndex :type Integer) (bFromSweep :type Boolean) (SweepResult :type Hit%20Result%20Structure%20%28by%20ref%29))
  (if (Components|ComponentHasTag OtherComp "PlayerCapsule")
    (bind _asbp_third_person_character (Utilities|Casting|CastToBP_ThirdPersonCharacter OtherActor))
    (if (not (Variables|/Game/ThirdPerson/Blueprints/BP_ThirdPersonCharacter.BP_ThirdPersonCharacter_C|GetIsPlayerDeconnected _asbp_third_person_character))
      (Variables|/Game/ThirdPerson/Blueprints/BP_ThirdPersonCharacter.BP_ThirdPersonCharacter_C|SetIsPlayerDeconnected _asbp_third_person_character true)
      (Default|DisconnectPlayer _asbp_third_person_character))))

(event Custom|PlayStartClose
  (Components|Timeline|SetPlayRate (Variables|Default|GetTLCLose) (/ 1.0 (Variables|Default|GetTL_CloseRate)))
  (Variables|Default|SetIsPlayingTL true)
  (Utilities|FlowControl|Delay (Variables|Default|GetWaitBeforeClose))
  (bind _open_close (Timeline|TLCLose PlayFromStart)
    (:Update
      (Transformation|SetActorLocation (Math|Vector|Lerp(Vector) (Variables|Default|GetFinal_Location) (Variables|Default|GetBaseLocation) _open_close) false false))
    (:Finished
      (Variables|Default|SetIsPlayingTL false)
      (Variables|Default|SetIs%20open false)
      (if (Variables|Default|GetLoop)
        (CallFunction|PlayStartOpen)))))

(event Custom|PlayStartOpen
  (Components|Timeline|SetPlayRate (Variables|Default|GetTLOpen) (/ 1.0 (Variables|Default|GetTL_OpenRate)))
  (Variables|Default|SetIsPlayingTL true)
  (Utilities|FlowControl|Delay (Variables|Default|GetWaitBeforeOpen))
  (bind _open_close (Timeline|TLOpen PlayFromStart)
    (:Update
      (Transformation|SetActorLocation (Math|Vector|Lerp(Vector) (Variables|Default|GetBaseLocation) (Variables|Default|GetFinal_Location) _open_close) false false))
    (:Finished
      (Variables|Default|SetIsPlayingTL false)
      (Variables|Default|SetIs%20open true)
      (if (Variables|Default|GetLoop)
        (CallFunction|PlayStartClose)))))

(event EventBeginPlay
  (bind _target__location (Variables|Default|GetTarget_%20Location))
  (Variables|Default|SetBaseLocation (Transformation|GetActorLocation))
  (if (Utilities|IsValid _target__location)
    (Variables|Default|SetFinal_Location (Transformation|GetActorLocation _target__location))))

(event EventOpen
  (if (not (Variables|Default|GetIs%20open))
    (Components|Timeline|SetPlayRate (Variables|Default|GetTLOpen) (/ 1.0 (Variables|Default|GetTL_OpenRate)))
    (Variables|Default|SetIsPlayingTL true)
    (Utilities|FlowControl|Delay (Variables|Default|GetWaitBeforeOpen))
    (bind _open_close (Timeline|TLOpen PlayFromStart)
      (:Update
        (Transformation|SetActorLocation (Math|Vector|Lerp(Vector) (Variables|Default|GetBaseLocation) (Variables|Default|GetFinal_Location) _open_close) false false))
      (:Finished
        (Variables|Default|SetIsPlayingTL false)
        (Variables|Default|SetIs%20open true)
        (if (Variables|Default|GetLoop)
          (CallFunction|PlayStartClose))))))

(event EventClose
  (if (Variables|Default|GetIs%20open)
    (Components|Timeline|SetPlayRate (Variables|Default|GetTLCLose) (/ 1.0 (Variables|Default|GetTL_CloseRate)))
    (Variables|Default|SetIsPlayingTL true)
    (Utilities|FlowControl|Delay (Variables|Default|GetWaitBeforeClose))
    (bind _open_close (Timeline|TLCLose PlayFromStart)
      (:Update
        (Transformation|SetActorLocation (Math|Vector|Lerp(Vector) (Variables|Default|GetFinal_Location) (Variables|Default|GetBaseLocation) _open_close) false false))
      (:Finished
        (Variables|Default|SetIsPlayingTL false)
        (Variables|Default|SetIs%20open false)
        (if (Variables|Default|GetLoop)
          (CallFunction|PlayStartOpen))))))

(fn ConstructionScript
  (Transformation|SetWorldScale3D (Variables|Default|GetDeath-Zone) (Variables|Default|GetScale-Death%20zone)))