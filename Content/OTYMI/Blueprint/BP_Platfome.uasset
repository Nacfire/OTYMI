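; BP_Platfome is a configurable platform actor whose mesh, scale and cable interaction are driven by variables.
; The construction script applies StaticMesh and Scale to the Mesh component.
; On BeginPlay, CableCanOverlap switches the mesh's collision object type between a custom channel (GameTraceChannel1) and WorldDynamic.
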(event EventBeginPlay
  (if (Variables|Default|GetCable_Can_Overlap)
    (Collision|SetCollisionObjectType (Variables|Default|GetMesh) "ECC_GameTraceChannel1")
    (else
      (Collision|SetCollisionObjectType (Variables|Default|GetMesh) "ECC_WorldDynamic"))))

(event Collision|EventActorBeginOverlap
  (params (OtherActor :type Actor%20Object%20Reference)))

(event EventTick
  (params (DeltaSeconds :type Float%20%28single-precision%29)))

(fn ConstructionScript
  (Components|StaticMesh|SetStaticMesh (Variables|Default|GetMesh) (Variables|Default|GetStatic_Mesh))
  (Transformation|SetWorldScale3D (Variables|Default|GetMesh) (Variables|Default|GetScale)))