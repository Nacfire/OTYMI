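; BP_MovePointOnCameraSpline is a trigger volume that reshapes a referenced camera spline when enough players stand inside it.
; The Box, scaled in the construction script, counts overlapping PlayerCapsule-tagged components and fires when the count equals NeedNumberOfPlayer.
; Activation adds Zoffset to the local height of the listed spline points.
; Activate flips on each firing, so only every other one moves points, cumulatively and without restoring them.
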(event OnComponentBeginOverlap(Box)
  (params (OverlappedComponent :type Primitive%20Component%20Object%20Reference) (OtherActor :type Actor%20Object%20Reference) (OtherComp :type Primitive%20Component%20Object%20Reference) (OtherBodyIndex :type Integer) (bFromSweep :type Boolean) (SweepResult :type Hit%20Result%20Structure%20%28by%20ref%29))
  (if (Components|ComponentHasTag OtherComp "PlayerCapsule")
    (Variables|Default|SetNumber%20of%20player (+ (Variables|Default|GetNumber%20of%20player) 1))
    (if (== (Variables|Default|GetNumber%20of%20player) (Variables|Default|GetNeed%20number%20of%20player))
      (CallFunction|MovePointonSpline))))

(event OnComponentEndOverlap(Box)
  (params (OverlappedComponent :type Primitive%20Component%20Object%20Reference) (OtherActor :type Actor%20Object%20Reference) (OtherComp :type Primitive%20Component%20Object%20Reference) (OtherBodyIndex :type Integer))
  (if (Components|ComponentHasTag OtherComp "PlayerCapsule")
    (Variables|Default|SetNumber%20of%20player (- (Variables|Default|GetNumber%20of%20player) 1))
    (if (<= (Variables|Default|GetNumber%20of%20player) 0)
      (Variables|Default|SetNumber%20of%20player 0))))

(event Custom|Move%20Point%20On%20Spline
  (if (Variables|Default|GetActivate)
    (Variables|Default|SetActivate (not (Variables|Default|GetActivate)))
    (else
      (Variables|Default|SetActivate true)
      (for _array_element (Variables|Default|GetPointOnSplineIndex)
        (Spline|SetLocationatSplinePoint (Variables|/Game/OTYMI/Blueprint/Bp_CameraSpline.Bp_CameraSpline_C|GetCam%20Spline (Variables|Default|GetSpline)) _array_element (+ (Spline|GetLocationatSplinePoint (Variables|/Game/OTYMI/Blueprint/Bp_CameraSpline.Bp_CameraSpline_C|GetCam%20Spline (Variables|Default|GetSpline)) _array_element "Local") (Math|Vector|MakeVector 0.0 0.0 (Variables|Default|GetZoffset))) "Local" true)))))

(event EventBeginPlay)

(event Collision|EventActorBeginOverlap
  (params (OtherActor :type Actor%20Object%20Reference)))

(event EventTick
  (params (DeltaSeconds :type Float%20%28single-precision%29)))

(fn ConstructionScript
  (Transformation|SetWorldScale3D (Variables|Default|GetBox) (Variables|Default|GetScale%20Trigger)))