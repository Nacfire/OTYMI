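; Configurable moving platform that slides between its base position and FinalLocation through Open and Close events, optionally looping.
; Timelines lerp the mesh after a delay, at adjustable rates.
; An optional trigger enables physics on tagged falling platforms until a looping timer sees them stop, and calls DisconnectPlayer on the player character.
; The construction script applies mesh, material and scales, offsetting mesh and trigger from bounds height.
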(event OnComponentBeginOverlap(Triggerphysics)
  (params (OverlappedComponent :type Primitive%20Component%20Object%20Reference) (OtherActor :type Actor%20Object%20Reference) (OtherComp :type Primitive%20Component%20Object%20Reference) (OtherBodyIndex :type Integer) (bFromSweep :type Boolean) (SweepResult :type Hit%20Result%20Structure%20%28by%20ref%29))
  (if (Actor|ActorHasTag OtherActor "CanPhysics")
    (if (Variables|Default|GetUse_TriggerPhysics)
      (bind _asbp_platform_fall (Utilities|Casting|CastToBP_PlatformFall OtherActor))
      (Physics|SetSimulatePhysics (Variables|/Game/OTYMI/Buton_et_interactible/BP_PlatformFall.BP_PlatformFall_C|GetMesh _asbp_platform_fall) true)
      (if (Utilities|Time|IsValidTimerHandle (Variables|Default|GetTimerRef))
        (Utilities|Time|UnpauseTimerbyHandle (Variables|Default|GetTimerRef))
        (else
          (bind _returnvalue (Utilities|Time|SetTimerbyEvent (delegate Custom|Check%20velocity%20Ref) 0.01 true))
          (Variables|Default|SetTimerRef _returnvalue))))
    (elif (Components|ComponentHasTag OtherComp "PlayerCapsule")
      (if (Variables|Default|GetUse_TriggerPhysics)
        (bind _asbp_third_person_character (Utilities|Casting|CastToBP_ThirdPersonCharacter (Components|GetOwner OtherComp)))
        (Default|DisconnectPlayer _asbp_third_person_character)))))

(event Custom|Check%20velocity%20Ref
  (if (Utilities|Operators|EqualEqual :A (Transformation|GetVelocity (stale OnComponentBeginOverlap(Triggerphysics) _asbp_platform_fall)) :ErrorTolerance 1.0)
    (Physics|SetSimulatePhysics (Variables|/Game/OTYMI/Buton_et_interactible/BP_PlatformFall.BP_PlatformFall_C|GetMesh (stale OnComponentBeginOverlap(Triggerphysics) _asbp_platform_fall)) false)
    (Utilities|Time|PauseTimerbyHandle (Variables|Default|GetTimerRef))))

(event Custom|PlayStartClose
  (bind _static_mesh (Variables|Default|GetStatic_mesh))
  (bind _scalemesh (Variables|Default|GetScaleMesh))
  (bind _returnvalue (StaticMesh|GetBoundingBox _static_mesh))
  (bind _returnvalue_2 (- (.max _returnvalue) (.min _returnvalue)))
  (bind _returnvalue_3 (* (.z _returnvalue_2) (.z _scalemesh)))
  (bind _returnvalue_4 (/ _returnvalue_3 2.0))
  (Components|Timeline|SetPlayRate (Variables|Default|GetTLClose) (/ 1.0 (Variables|Porte_coulisante|GetTL_CloseRate)))
  (Variables|Default|SetIsPlayingTL true)
  (Utilities|FlowControl|Delay (Variables|Porte_coulisante|GetWaitBeforeClose))
  (bind _open_close (Timeline|TLClose PlayFromStart)
    (:Update
      (Transformation|SetRelativeLocationAndRotation (Variables|Default|GetMesh) (Math|Vector|Lerp(Vector) (+ (Variables|Porte_coulisante|GetFinal_Location) (Math|Vector|MakeVector 0.0 0.0 _returnvalue_4)) (Math|Vector|MakeVector 0.0 0.0 _returnvalue_4) _open_close) "0, 0, 0" false false))
    (:Finished
      (Variables|Default|SetIsPlayingTL false)
      (Variables|Default|SetIs%20open false)
      (if (Variables|Porte_coulisante|GetLoop)
        (CallFunction|PlayStartOpen)))))

(event Custom|PlayStartOpen
  (bind _static_mesh (Variables|Default|GetStatic_mesh))
  (bind _scalemesh (Variables|Default|GetScaleMesh))
  (bind _returnvalue (StaticMesh|GetBoundingBox _static_mesh))
  (bind _returnvalue_2 (- (.max _returnvalue) (.min _returnvalue)))
  (bind _returnvalue_3 (* (.z _returnvalue_2) (.z _scalemesh)))
  (bind _returnvalue_4 (/ _returnvalue_3 2.0))
  (Components|Timeline|SetPlayRate (Variables|Default|GetTL_Open) (/ 1.0 (Variables|Porte_coulisante|GetTL_OpenRate)))
  (Variables|Default|SetIsPlayingTL true)
  (Utilities|FlowControl|Delay (Variables|Porte_coulisante|GetWaitBeforeOpen))
  (bind _open_close (Timeline|TL_Open PlayFromStart)
    (:Update
      (Transformation|SetRelativeLocationAndRotation (Variables|Default|GetMesh) (Math|Vector|Lerp(Vector) (Math|Vector|MakeVector 0.0 0.0 _returnvalue_4) (+ (Variables|Porte_coulisante|GetFinal_Location) (Math|Vector|MakeVector 0.0 0.0 _returnvalue_4)) _open_close) "0, 0, 0" false false))
    (:Finished
      (Variables|Default|SetIsPlayingTL false)
      (Variables|Default|SetIs%20open true)
      (if (Variables|Porte_coulisante|GetLoop)
        (CallFunction|PlayStartClose)))))

(event EventBeginPlay)

(event Collision|EventActorBeginOverlap
  (params (OtherActor :type Actor%20Object%20Reference)))

(event EventTick
  (params (DeltaSeconds :type Float%20%28single-precision%29)))

(event EventOpen
  (bind _static_mesh (Variables|Default|GetStatic_mesh))
  (bind _scalemesh (Variables|Default|GetScaleMesh))
  (bind _returnvalue (StaticMesh|GetBoundingBox _static_mesh))
  (bind _returnvalue_2 (- (.max _returnvalue) (.min _returnvalue)))
  (bind _returnvalue_3 (* (.z _returnvalue_2) (.z _scalemesh)))
  (bind _returnvalue_4 (/ _returnvalue_3 2.0))
  (if (not (Variables|Default|GetIs%20open))
    (Components|Timeline|SetPlayRate (Variables|Default|GetTL_Open) (/ 1.0 (Variables|Porte_coulisante|GetTL_OpenRate)))
    (Variables|Default|SetIsPlayingTL true)
    (Utilities|FlowControl|Delay (Variables|Porte_coulisante|GetWaitBeforeOpen))
    (bind _open_close (Timeline|TL_Open PlayFromStart)
      (:Update
        (Transformation|SetRelativeLocationAndRotation (Variables|Default|GetMesh) (Math|Vector|Lerp(Vector) (Math|Vector|MakeVector 0.0 0.0 _returnvalue_4) (+ (Variables|Porte_coulisante|GetFinal_Location) (Math|Vector|MakeVector 0.0 0.0 _returnvalue_4)) _open_close) "0, 0, 0" false false))
      (:Finished
        (Variables|Default|SetIsPlayingTL false)
        (Variables|Default|SetIs%20open true)
        (if (Variables|Porte_coulisante|GetLoop)
          (CallFunction|PlayStartClose))))))

(event EventClose
  (bind _static_mesh (Variables|Default|GetStatic_mesh))
  (bind _scalemesh (Variables|Default|GetScaleMesh))
  (bind _returnvalue (StaticMesh|GetBoundingBox _static_mesh))
  (bind _returnvalue_2 (- (.max _returnvalue) (.min _returnvalue)))
  (bind _returnvalue_3 (* (.z _returnvalue_2) (.z _scalemesh)))
  (bind _returnvalue_4 (/ _returnvalue_3 2.0))
  (if (Variables|Default|GetIs%20open)
    (Components|Timeline|SetPlayRate (Variables|Default|GetTLClose) (/ 1.0 (Variables|Porte_coulisante|GetTL_CloseRate)))
    (Variables|Default|SetIsPlayingTL true)
    (Utilities|FlowControl|Delay (Variables|Porte_coulisante|GetWaitBeforeClose))
    (bind _open_close (Timeline|TLClose PlayFromStart)
      (:Update
        (Transformation|SetRelativeLocationAndRotation (Variables|Default|GetMesh) (Math|Vector|Lerp(Vector) (+ (Variables|Porte_coulisante|GetFinal_Location) (Math|Vector|MakeVector 0.0 0.0 _returnvalue_4)) (Math|Vector|MakeVector 0.0 0.0 _returnvalue_4) _open_close) "0, 0, 0" false false))
      (:Finished
        (Variables|Default|SetIsPlayingTL false)
        (Variables|Default|SetIs%20open false)
        (if (Variables|Porte_coulisante|GetLoop)
          (CallFunction|PlayStartOpen))))))

(fn ConstructionScript
  (bind _static_mesh (Variables|Default|GetStatic_mesh))
  (bind _trigger_physics (Variables|Default|GetTrigger%20physics))
  (bind _scalemesh (Variables|Default|GetScaleMesh))
  (bind _static_mesh_2 (Variables|Default|GetStatic_mesh))
  (bind _returnvalue (StaticMesh|GetBoundingBox _static_mesh))
  (bind _returnvalue_2 (Components|Box|GetScaledBoxExtent _trigger_physics))
  (bind _returnvalue_3 (StaticMesh|GetBoundingBox _static_mesh_2))
  (bind _z (Math|Vector|BreakVector _scalemesh))
  (bind _z_2 (Math|Vector|BreakVector _returnvalue_2))
  (Components|StaticMesh|SetStaticMesh (Variables|Default|GetMesh) (Variables|Default|GetStatic_mesh))
  (Rendering|Material|SetMaterial (Variables|Default|GetMesh) 0 (Variables|Default|GetMaterial))
  (Transformation|SetWorldScale3D (Variables|Default|GetTrigger%20physics) (Variables|Default|GetScaleTriger))
  (Transformation|SetWorldScale3D (Variables|Default|GetMesh) (Variables|Default|GetScaleMesh))
  (Transformation|SetRelativeLocation (Variables|Default|GetMesh) (Math|Vector|MakeVector 0.0 0.0 (/ (* (.z (- (.max _returnvalue) (.min _returnvalue))) (.z (Variables|Default|GetScaleMesh))) 2.0)) false false)
  (Transformation|SetRelativeLocation (Variables|Default|GetTrigger%20physics) (Math|Vector|MakeVector 0.0 0.0 (Utilities|Operators|Divide (+ _z_2 (- _z_2 (* (.z (- (.max _returnvalue_3) (.min _returnvalue_3))) _z))) 2.0 _z)) false false))