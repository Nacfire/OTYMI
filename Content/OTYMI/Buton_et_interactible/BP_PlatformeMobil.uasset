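; Moving platform that slides between its start location and a referenced end-point actor, optionally looping.
; Open and Close events run delayed timelines that lerp the actor's location at configurable rates.
; An optional trigger enables physics on overlapping tagged BP_Platform-fall actors until a polling timer finds them at rest, and calls DisconnectPlayer on player capsules.
; The construction script applies mesh, material and scales, placing the trigger above the mesh.
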(event OnComponentBeginOverlap(Triggerphysics)
  (params (OverlappedComponent :type Primitive%20Component%20Object%20Reference) (OtherActor :type Actor%20Object%20Reference) (OtherComp :type Primitive%20Component%20Object%20Reference) (OtherBodyIndex :type Integer) (bFromSweep :type Boolean) (SweepResult :type Hit%20Result%20Structure%20%28by%20ref%29))
  (if (Actor|ActorHasTag OtherActor "CanPhysics")
    (if (Variables|Default|GetUse_TriggerPhysics)
      (bind _asbp_platform_fall (Utilities|Casting|CastToBP_Platform-fall OtherActor))
      (Physics|SetSimulatePhysics (Variables|/Game/OTYMI/Buton_et_interactible/BP_Platform-fall.BP_Platform-fall_C|GetMesh _asbp_platform_fall) true)
      (if (Utilities|Time|IsValidTimerHandle (Variables|Default|GetTimerRef))
        (Utilities|Time|UnpauseTimerbyHandle (Variables|Default|GetTimerRef))
        (else
          (bind _returnvalue (Utilities|Time|SetTimerbyEvent (delegate Custom|Check%20velocity%20Ref) 0.01 true))
          (Variables|Default|SetTimerRef _returnvalue))))
    (elif (Components|ComponentHasTag OtherComp "PlayerCapsule")
      (if (Variables|Default|GetUse_TriggerPhysics)
        (bind _asbp_third_person_character (Utilities|Casting|CastToBP_ThirdPersonCharacter (Components|GetOwner OtherComp)))
        (Default|DisconnectPlayer _asbp_third_person_character)))))

(event Custom|Check%20velocity%20Ref
  (if (Utilities|Operators|EqualEqual :A (Transformation|GetVelocity (stale OnComponentBeginOverlap(Triggerphysics) _asbp_platform_fall)) :ErrorTolerance 1.0)
    (Physics|SetSimulatePhysics (Variables|/Game/OTYMI/Buton_et_interactible/BP_Platform-fall.BP_Platform-fall_C|GetMesh (stale OnComponentBeginOverlap(Triggerphysics) _asbp_platform_fall)) false)
    (Utilities|Time|PauseTimerbyHandle (Variables|Default|GetTimerRef))))

(event Custom|PlayStartClose
  (Components|Timeline|SetPlayRate (Variables|Default|GetTLClose) (/ 1.0 (Variables|Porte_coulisante|GetTL_CloseRate)))
  (Variables|Default|SetIsPlayingTL true)
  (Utilities|FlowControl|Delay (Variables|Porte_coulisante|GetWaitBeforeClose))
  (bind _open_close (Timeline|TLClose PlayFromStart)
    (:Update
      (Transformation|SetActorLocation (Math|Vector|Lerp(Vector) (Variables|Porte_coulisante|GetFinal_Location) (Variables|Default|GetBackupBasePose) _open_close) false false))
    (:Finished
      (Variables|Default|SetIsPlayingTL false)
      (Variables|Default|SetIs%20open false)
      (if (Variables|Porte_coulisante|GetLoop)
        (CallFunction|PlayStartOpen)))))

(event Custom|PlayStartOpen
  (Components|Timeline|SetPlayRate (Variables|Default|GetTL_Open) (/ 1.0 (Variables|Porte_coulisante|GetTL_OpenRate)))
  (Variables|Default|SetIsPlayingTL true)
  (Utilities|FlowControl|Delay (Variables|Porte_coulisante|GetWaitBeforeOpen))
  (bind _open_close (Timeline|TL_Open PlayFromStart)
    (:Update
      (Transformation|SetActorLocation (Math|Vector|Lerp(Vector) (Variables|Default|GetBackupBasePose) (Variables|Porte_coulisante|GetFinal_Location) _open_close) false false))
    (:Finished
      (Variables|Default|SetIsPlayingTL false)
      (Variables|Default|SetIs%20open true)
      (if (Variables|Porte_coulisante|GetLoop)
        (CallFunction|PlayStartClose)))))

(event EventBeginPlay
  (bind _refendpoint (Variables|Porte_coulisante|GetRefEndPoint))
  (Variables|Default|SetBackupBasePose (Transformation|GetActorLocation))
  (if (Utilities|IsValid _refendpoint)
    (Variables|Porte_coulisante|SetFinal_Location (Transformation|GetActorLocation _refendpoint))))

(event EventOpen
  (bind _refendpoint (Variables|Porte_coulisante|GetRefEndPoint))
  (if (not (Variables|Default|GetIs%20open))
    (Variables|Default|SetBackupBasePose (Transformation|GetActorLocation))
    (if (Utilities|IsValid _refendpoint)
      (Variables|Porte_coulisante|SetFinal_Location (Transformation|GetActorLocation _refendpoint))
      (Components|Timeline|SetPlayRate (Variables|Default|GetTL_Open) (/ 1.0 (Variables|Porte_coulisante|GetTL_OpenRate)))
      (Variables|Default|SetIsPlayingTL true)
      (Utilities|FlowControl|Delay (Variables|Porte_coulisante|GetWaitBeforeOpen))
      (bind _open_close (Timeline|TL_Open PlayFromStart)
        (:Update
          (Transformation|SetActorLocation (Math|Vector|Lerp(Vector) (Variables|Default|GetBackupBasePose) (Variables|Porte_coulisante|GetFinal_Location) _open_close) false false))
        (:Finished
          (Variables|Default|SetIsPlayingTL false)
          (Variables|Default|SetIs%20open true)
          (if (Variables|Porte_coulisante|GetLoop)
            (CallFunction|PlayStartClose)))))))

(event EventClose
  (bind _refendpoint (Variables|Porte_coulisante|GetRefEndPoint))
  (if (Variables|Default|GetIs%20open)
    (Variables|Default|SetBackupBasePose (Transformation|GetActorLocation))
    (if (Utilities|IsValid _refendpoint)
      (Variables|Porte_coulisante|SetFinal_Location (Transformation|GetActorLocation _refendpoint))
      (Components|Timeline|SetPlayRate (Variables|Default|GetTLClose) (/ 1.0 (Variables|Porte_coulisante|GetTL_CloseRate)))
      (Variables|Default|SetIsPlayingTL true)
      (Utilities|FlowControl|Delay (Variables|Porte_coulisante|GetWaitBeforeClose))
      (bind _open_close (Timeline|TLClose PlayFromStart)
        (:Update
          (Transformation|SetActorLocation (Math|Vector|Lerp(Vector) (Variables|Porte_coulisante|GetFinal_Location) (Variables|Default|GetBackupBasePose) _open_close) false false))
        (:Finished
          (Variables|Default|SetIsPlayingTL false)
          (Variables|Default|SetIs%20open false)
          (if (Variables|Porte_coulisante|GetLoop)
            (CallFunction|PlayStartOpen)))))))

(fn ConstructionScript
  (Components|StaticMesh|SetStaticMesh (Variables|Default|GetMesh) (Variables|Default|GetStatic_mesh))
  (Rendering|Material|SetMaterial (Variables|Default|GetMesh) 0 (Variables|Default|GetMaterial))
  (Transformation|SetWorldScale3D (Variables|Default|GetTrigger%20physics) (Variables|Default|GetScaleTriger))
  (Transformation|SetWorldScale3D (Variables|Default|GetMesh) (Variables|Default|GetScaleMesh))
  (Transformation|SetWorldLocation (Variables|Default|GetTrigger%20physics) (+ (Transformation|GetWorldLocation (Variables|Default|GetMesh)) (Math|Vector|MakeVector 0.0 0.0 (.Z (Math|Vector|BreakVector (Components|Box|GetScaledBoxExtent (Variables|Default|GetTrigger%20physics)))))) false false))