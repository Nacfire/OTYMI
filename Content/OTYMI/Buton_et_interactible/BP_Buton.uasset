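; Pressure plate button that activates linked interactibles once every button in its ButonList is pressed.
; A trigger counts PlayerCapsule overlaps, then opens disconnect zones or a moving or rotating platform through BPIButon_To_Interractible, or enables physics, optionally frozen by a velocity-polling timer once at rest.
; With ExitPlaqueDePretion, emptying the plate deactivates it and closes its platform.
; A looping timer lights the activation feedback; construction sets visuals and layout.
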(event OnComponentBeginOverlap(Trigger)
  (params (OverlappedComponent :type Primitive%20Component%20Object%20Reference) (OtherActor :type Actor%20Object%20Reference) (OtherComp :type Primitive%20Component%20Object%20Reference) (OtherBodyIndex :type Integer) (bFromSweep :type Boolean) (SweepResult :type Hit%20Result%20Structure%20%28by%20ref%29))
  (bind _movingplatform (Variables|Mouvingandrotate|GetMovingPlatform))
  (bind _rotateplatform (Variables|Mouvingandrotate|GetRotatePlatform))
  (if (Components|ComponentHasTag OtherComp "PlayerCapsule")
    (Variables|Default|SetConteurJoueur (+ (Variables|Default|GetConteurJoueur) 1))
    (if (not (> (Variables|Default|GetConteurJoueur) 1))
      (if (not (Variables|Default|GetActivate))
        (Variables|Default|SetActivate true)
        (Variables|Default|SetConteurPlack%20activer 0)
        (for _array_element (Variables|Default|GetButonList)
          (if (Variables|BP_Buton_C|GetActivate _array_element)
            (Variables|Default|SetConteurPlack%20activer (+ (Variables|Default|GetConteurPlack%20activer) 1))))
        (if (== (Variables|Default|GetConteurPlack%20activer) (Utilities|Array|Length (Variables|Default|GetButonList)))
          (if (Variables|Default|GetUseDisconectZoneMobil)
            (for _array_element_2 (Variables|Default|GetDisconectZoneRef)
              (if (Utilities|DoesObjectImplementInterface _array_element_2 "/Game/OTYMI/Buton_et_interactible/BPIButon_To_Interractible.BPIButon_To_Interractible_C")
                (if (not (Variables|/Game/OTYMI/Blueprint/BP_Disconect-Zone_Mobil.BP_Disconect-Zone_Mobil_C|GetIsPlayingTL _array_element_2))
                  (if (not (Variables|/Game/OTYMI/Blueprint/BP_Disconect-Zone_Mobil.BP_Disconect-Zone_Mobil_C|GetIs%20open _array_element_2))
                    (Class|BPIButontoInterractible|Open(Message) _array_element_2)))))
            (elif (Variables|Default|GetUse%20physics)
              (Physics|SetSimulatePhysics (Variables|/Game/OTYMI/Buton_et_interactible/BP_Platform-fall.BP_Platform-fall_C|GetMesh (Variables|Physics|GetInteractible)) true)
              (if (Variables|Physics|GetDestoy%20afer%20Get%20physique)
                (if (Utilities|Time|IsValidTimerHandle (Variables|Default|GetTimerRef))
                  (Utilities|Time|UnpauseTimerbyHandle (Variables|Default|GetTimerRef))
                  (else
                    (bind _returnvalue (Utilities|Time|SetTimerbyEvent (delegate Custom|Check%20velocity%20Ref) 0.01 true))
                    (Variables|Default|SetTimerRef _returnvalue))))
              (elif (Variables|Mouvingandrotate|GetMoving)
                (if (Utilities|DoesObjectImplementInterface _movingplatform "/Game/OTYMI/Buton_et_interactible/BPIButon_To_Interractible.BPIButon_To_Interractible_C")
                  (if (not (Variables|/Game/OTYMI/Buton_et_interactible/BP_PlatformeMobil.BP_PlatformeMobil_C|GetIsPlayingTL _movingplatform))
                    (if (not (Variables|/Game/OTYMI/Buton_et_interactible/BP_PlatformeMobil.BP_PlatformeMobil_C|GetIs%20open _movingplatform))
                      (Class|BPIButontoInterractible|Open(Message) _movingplatform))))
                (elif (Utilities|DoesObjectImplementInterface _rotateplatform "/Game/OTYMI/Buton_et_interactible/BPIButon_To_Interractible.BPIButon_To_Interractible_C")
                  (if (not (Variables|/Game/OTYMI/Buton_et_interactible/BP_PlatformeRotate.BP_PlatformeRotate_C|GetIsPlayingTL _rotateplatform))
                    (if (not (Variables|/Game/OTYMI/Buton_et_interactible/BP_PlatformeRotate.BP_PlatformeRotate_C|GetIs%20open _rotateplatform))
                      (Class|BPIButontoInterractible|Open(Message) _rotateplatform))))))))))))

(event OnComponentEndOverlap(Trigger)
  (params (OverlappedComponent :type Primitive%20Component%20Object%20Reference) (OtherActor :type Actor%20Object%20Reference) (OtherComp :type Primitive%20Component%20Object%20Reference) (OtherBodyIndex :type Integer))
  (bind _movingplatform (Variables|Mouvingandrotate|GetMovingPlatform))
  (bind _rotateplatform (Variables|Mouvingandrotate|GetRotatePlatform))
  (if (Components|ComponentHasTag OtherComp "PlayerCapsule")
    (Variables|Default|SetConteurJoueur (- (Variables|Default|GetConteurJoueur) 1))
    (if (<= (Variables|Default|GetConteurJoueur) 0)
      (if (Variables|Default|GetExit%20plaque%20de%20pretion)
        (if (Variables|Mouvingandrotate|GetMoving)
          (if (Utilities|DoesObjectImplementInterface _movingplatform "/Game/OTYMI/Buton_et_interactible/BPIButon_To_Interractible.BPIButon_To_Interractible_C")
            (Variables|Default|SetConteurPlack%20activer 0)
            (Variables|Default|SetActivate false)
            (if (not (Variables|/Game/OTYMI/Buton_et_interactible/BP_PlatformeMobil.BP_PlatformeMobil_C|GetIsPlayingTL _movingplatform))
              (if (Variables|/Game/OTYMI/Buton_et_interactible/BP_PlatformeMobil.BP_PlatformeMobil_C|GetIs%20open _movingplatform)
                (Class|BPIButontoInterractible|Close(Message) _movingplatform)
                (Variables|Default|SetConteurJoueur 0))))
          (elif (Utilities|DoesObjectImplementInterface _rotateplatform "/Game/OTYMI/Buton_et_interactible/BPIButon_To_Interractible.BPIButon_To_Interractible_C")
            (Variables|Default|SetConteurPlack%20activer 0)
            (Variables|Default|SetActivate false)
            (if (not (Variables|/Game/OTYMI/Buton_et_interactible/BP_PlatformeRotate.BP_PlatformeRotate_C|GetIsPlayingTL _rotateplatform))
              (if (Variables|/Game/OTYMI/Buton_et_interactible/BP_PlatformeRotate.BP_PlatformeRotate_C|GetIs%20open _rotateplatform)
                (Class|BPIButontoInterractible|Close(Message) _rotateplatform)
                (Variables|Default|SetConteurJoueur 0)))))))))

(event Custom|Check%20velocity%20Ref
  (if (Utilities|Operators|EqualEqual :A (Transformation|GetVelocity (Variables|Physics|GetInteractible)) :ErrorTolerance 1.0)
    (Physics|SetSimulatePhysics (Variables|/Game/OTYMI/Buton_et_interactible/BP_Platform-fall.BP_Platform-fall_C|GetMesh (Variables|Physics|GetInteractible)) false)
    (Utilities|Time|PauseTimerbyHandle (Variables|Default|GetTimerRef))))

(event Custom|Feed%20back%20activation
  (if (Variables|Default|GetActivate)
    (Rendering|Components|Light|SetIntensity (Variables|Default|GetPointLight) (Variables|Feedback|GetLight%20Inencity))
    (Utilities|Time|PauseTimerbyHandle (Variables|Default|GetTimer%20feed%20back))))

(event EventBeginPlay)

(event Collision|EventActorBeginOverlap
  (params (OtherActor :type Actor%20Object%20Reference))
  (bind _returnvalue (Utilities|Time|SetTimerbyEvent (delegate Custom|Feed%20back%20activation) 0.1 true))
  (Variables|Default|SetTimer%20feed%20back _returnvalue))

(event EventTick
  (params (DeltaSeconds :type Float%20%28single-precision%29)))

(fn ConstructionScript
  (bind _sm_visuel (Variables|Default|GetSM_visuel))
  (bind _scalebuton (Variables|Default|GetScaleButon))
  (bind _returnvalue (StaticMesh|GetBoundingBox _sm_visuel))
  (bind _returnvalue_2 (- (.max _returnvalue) (.min _returnvalue)))
  (bind _returnvalue_3 (* _returnvalue_2 _scalebuton))
  (Components|StaticMesh|SetStaticMesh (Variables|Default|GetSM_Buton) (Variables|Default|GetSM_visuel))
  (Rendering|Material|SetMaterial (Variables|Default|GetSM_Buton) 0 (Variables|Default|GetMaterial))
  (Transformation|SetWorldScale3D (Variables|Default|GetTrigger) (Variables|Default|GetScaleTriger))
  (Transformation|SetWorldScale3D (Variables|Default|GetSM_Buton) (Variables|Default|GetScaleButon))
  (Transformation|SetWorldLocation (Variables|Default|GetTrigger) (+ (Transformation|GetWorldLocation (Variables|Default|GetSM_Buton)) (Math|Vector|MakeVector 0.0 0.0 (.Z (Math|Vector|BreakVector (Components|Box|GetScaledBoxExtent (Variables|Default|GetTrigger)))))) false false)
  (Transformation|SetRelativeLocation (Variables|Default|GetPointLight) (Math|Vector|MakeVector 0.0 0.0 (.z (+ _returnvalue_3 (/ _returnvalue_3 2.0)))) false false))