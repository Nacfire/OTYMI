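; Interactable switch actor that lets players in its trigger box open or close a linked moving or rotating platform.
; Overlapping player capsules are listed, and a fast looping timer polls each connected player's interact input, sending interface open/close messages when the platform is idle.
; Entering toggles Activate, which a second timer polls to set the point light's intensity.
; The construction script applies mesh, material and trigger size, placing the light from mesh bounds.
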(event OnComponentBeginOverlap(Zonzd'interaction)
  (params (OverlappedComponent :type Primitive%20Component%20Object%20Reference) (OtherActor :type Actor%20Object%20Reference) (OtherComp :type Primitive%20Component%20Object%20Reference) (OtherBodyIndex :type Integer) (bFromSweep :type Boolean) (SweepResult :type Hit%20Result%20Structure%20%28by%20ref%29))
  (if (Components|ComponentHasTag OtherComp "PlayerCapsule")
    (bind _asbp_third_person_character (Utilities|Casting|CastToBP_ThirdPersonCharacter OtherActor))
    (Utilities|Array|Add (Variables|Default|GetPlayerList) _asbp_third_person_character)
    (Variables|Default|SetActivate (not (Variables|Default|GetActivate)))
    (if (Utilities|Time|IsValidTimerHandle (Variables|Default|GetTimer%20Check%20to%20open))
      (Utilities|Time|UnpauseTimerbyHandle (Variables|Default|GetTimer%20Check%20to%20open))
      (else
        (bind _returnvalue (Utilities|Time|SetTimerbyEvent (delegate Custom|Check%20Input) 0.01 true true))
        (Variables|Default|SetTimer%20Check%20to%20open _returnvalue)))))

(event OnComponentEndOverlap(Zonzd'interaction)
  (params (OverlappedComponent :type Primitive%20Component%20Object%20Reference) (OtherActor :type Actor%20Object%20Reference) (OtherComp :type Primitive%20Component%20Object%20Reference) (OtherBodyIndex :type Integer))
  (if (Components|ComponentHasTag OtherComp "PlayerCapsule")
    (bind _asbp_third_person_character (Utilities|Casting|CastToBP_ThirdPersonCharacter OtherActor))
    (Utilities|Array|RemoveItem (Variables|Default|GetPlayerList) _asbp_third_person_character)
    (CallFunction|UpdateFeedback)
    (Utilities|Time|PauseTimerbyHandle (Variables|Default|GetTimer%20Check%20to%20open))))

(event Custom|Check%20Input
  (bind _rotateplatform (Variables|Default|GetRotatePlatform))
  (for _array_element (Variables|Default|GetPlayerList)
    (if (not (Variables|/Game/ThirdPerson/Blueprints/BP_ThirdPersonCharacter.BP_ThirdPersonCharacter_C|GetIsPlayerDeconnected _array_element))
      (if (Variables|/Game/ThirdPerson/Blueprints/BP_ThirdPersonCharacter.BP_ThirdPersonCharacter_C|GetInteractPress _array_element)
        (if (Variables|Default|GetMoving)
          (if (Utilities|DoesObjectImplementInterface (Variables|Default|GetMouvingPlatform) "/Game/OTYMI/Buton_et_interactible/BPIButon_To_Interractible.BPIButon_To_Interractible_C")
            (if (not (Variables|/Game/OTYMI/Buton_et_interactible/BP_PlatformeMobil.BP_PlatformeMobil_C|GetIsPlayingTL (Variables|Default|GetMouvingPlatform)))
              (if (Variables|/Game/OTYMI/Buton_et_interactible/BP_PlatformeMobil.BP_PlatformeMobil_C|GetIs%20open (Variables|Default|GetMouvingPlatform))
                (Class|BPIButontoInterractible|Close(Message) (Variables|Default|GetMouvingPlatform))
                (else
                  (Class|BPIButontoInterractible|Open(Message) (Variables|Default|GetMouvingPlatform))))))
          (elif (Utilities|DoesObjectImplementInterface _rotateplatform "/Game/OTYMI/Buton_et_interactible/BPIButon_To_Interractible.BPIButon_To_Interractible_C")
            (if (not (Variables|/Game/OTYMI/Buton_et_interactible/BP_PlatformeRotate.BP_PlatformeRotate_C|GetIsPlayingTL _rotateplatform))
              (if (Variables|/Game/OTYMI/Buton_et_interactible/BP_PlatformeRotate.BP_PlatformeRotate_C|GetIs%20open _rotateplatform)
                (Class|BPIButontoInterractible|Close(Message) _rotateplatform)
                (else
                  (Class|BPIButontoInterractible|Open(Message) _rotateplatform))))))))))

(event Custom|Feed%20back%20activation
  (if (Variables|Default|GetActivate)
    (Rendering|Components|Light|SetIntensity (Variables|Default|GetPointLight) (Variables|Feedback|GetLight%20Inencity))
    (Utilities|Time|PauseTimerbyHandle (Variables|Feedback|GetTimer%20feed%20back))))

(event Custom|UpdateFeedback
  (bind _returnvalue (Utilities|Time|SetTimerbyEvent (delegate Custom|Feed%20back%20activation) 0.1 true))
  (Variables|Feedback|SetTimer%20feed%20back _returnvalue))

(event EventBeginPlay
  (bind _returnvalue (Utilities|Time|SetTimerbyEvent (delegate Custom|Feed%20back%20activation) 0.1 true))
  (Variables|Feedback|SetTimer%20feed%20back _returnvalue))

(event Collision|EventActorBeginOverlap
  (params (OtherActor :type Actor%20Object%20Reference)))

(event EventTick
  (params (DeltaSeconds :type Float%20%28single-precision%29)))

(fn ConstructionScript
  (bind _mesh (Variables|Default|GetMesh))
  (bind _returnvalue (StaticMesh|GetBoundingBox _mesh))
  (bind _returnvalue_2 (- (.max _returnvalue) (.min _returnvalue)))
  (Components|StaticMesh|SetStaticMesh (Variables|Default|GetStaticMesh) (Variables|Default|GetMesh))
  (Rendering|Material|SetMaterial (Variables|Default|GetStaticMesh) 0 (Variables|Default|GetMaterial))
  (Components|Box|SetBoxExtent (Variables|Default|GetZonz%20d'interaction) (Variables|Default|GetScaleTriger) true)
  (Transformation|SetRelativeLocation (Variables|Default|GetPointLight) (Math|Vector|MakeVector 0.0 0.0 (.z (+ _returnvalue_2 (/ _returnvalue_2 2.0)))) false false))