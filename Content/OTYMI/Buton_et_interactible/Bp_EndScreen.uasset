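; BP_EndScreen is a trigger actor that runs the end sequence when a BP_ThirdPersonCharacter enters its box.
; The overlap fires only once, fading the first player's camera and audio out and holding the fade.
; It also sets CanMove to false on player characters 0 through 3.
; After a short delay, it adds the BPI_Fonduaunoir ("fade to black") widget to the viewport.
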(event OnComponentBeginOverlap(Box)
  (params (OverlappedComponent :type Primitive%20Component%20Object%20Reference) (OtherActor :type Actor%20Object%20Reference) (OtherComp :type Primitive%20Component%20Object%20Reference) (OtherBodyIndex :type Integer) (bFromSweep :type Boolean) (SweepResult :type Hit%20Result%20Structure%20%28by%20ref%29))
  (if (Class|GameplayStatics|ObjectIsA OtherActor "/Game/ThirdPerson/Blueprints/BP_ThirdPersonCharacter.BP_ThirdPersonCharacter_C")
    (Utilities|FlowControl|DoOnce false
      (:Completed
        (CameraFades|StartCameraFade :self (Game|GetPlayerCameraManager 0) :ToAlpha 1.0 :Duration 2.0 :bShouldFadeAudio true :bHoldWhenFinished true)
        (for _index (range 0 3)
          (Variables|/Game/ThirdPerson/Blueprints/BP_ThirdPersonCharacter.BP_ThirdPersonCharacter_C|SetCanMove? (.AsBP%20Third%20Person%20Character (Utilities|Casting|CastToBP_ThirdPersonCharacter (Game|GetPlayerCharacter _index))) false))
        (Utilities|FlowControl|Delay 2.5)
        (bind _returnvalue (UserInterface|CreateWidget "/Game/OTYMI/UI/BPI_Fondu-au-noir.BPI_Fondu-au-noir_C"))
        (UserInterface|Viewport|AddtoViewport _returnvalue 0)))))

(event EventBeginPlay)

(event Collision|EventActorBeginOverlap
  (params (OtherActor :type Actor%20Object%20Reference)))

(event EventTick
  (params (DeltaSeconds :type Float%20%28single-precision%29)))

(fn ConstructionScript)