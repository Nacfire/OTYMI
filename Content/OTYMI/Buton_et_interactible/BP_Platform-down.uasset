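; Platform actor that sinks while players stand on it and rises back to its starting height once they leave.
; Trigger overlaps with PlayerCapsule-tagged components update a player counter and enable Tick after a half-second delay.
; Tick moves the root down by a fixed per-frame step with no lower limit, or back up, disabling itself at the saved height.
; The construction script applies configurable mesh, material and scales, then positions mesh and trigger vertically.
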(event OnComponentBeginOverlap(TrigerPhysics)
  (params (OverlappedComponent :type Primitive%20Component%20Object%20Reference) (OtherActor :type Actor%20Object%20Reference) (OtherComp :type Primitive%20Component%20Object%20Reference) (OtherBodyIndex :type Integer) (bFromSweep :type Boolean) (SweepResult :type Hit%20Result%20Structure%20%28by%20ref%29))
  (if (Components|ComponentHasTag OtherComp "PlayerCapsule")
    (Variables|Default|SetCompteur_de_joueur (+ (Variables|Default|GetCompteur_de_joueur) 1))
    (if (> (Variables|Default|GetCompteur_de_joueur) 0)
      (Utilities|FlowControl|Delay 0.5)
      (Actor|Tick|SetActorTickEnabled true))))

(event OnComponentEndOverlap(TrigerPhysics)
  (params (OverlappedComponent :type Primitive%20Component%20Object%20Reference) (OtherActor :type Actor%20Object%20Reference) (OtherComp :type Primitive%20Component%20Object%20Reference) (OtherBodyIndex :type Integer))
  (if (Components|ComponentHasTag OtherComp "PlayerCapsule")
    (Variables|Default|SetCompteur_de_joueur (- (Variables|Default|GetCompteur_de_joueur) 1))))

(event EventBeginPlay
  (Variables|Default|SetBasePose (Transformation|GetWorldLocation (Variables|Default|GetDefaultSceneRoot))))

(event EventTick
  (params (DeltaSeconds :type Float%20%28single-precision%29))
  ;[1 0 0 0.5] Tick
  (if (> (Variables|Default|GetCompteur_de_joueur) 0)
    (Transformation|AddLocalOffset (Variables|Default|GetDefaultSceneRoot) (Math|Vector|MakeVector 0.0 0.0 -1.0) false false)
    (elif (Math|Float|NearlyEqual(Float) (.Z (Math|Vector|BreakVector (Variables|Default|GetBasePose))) (.Z (Math|Vector|BreakVector (Transformation|GetWorldLocation (Variables|Default|GetDefaultSceneRoot)))) 0.1)
      (Actor|Tick|SetActorTickEnabled false)
      (else
        (Transformation|AddLocalOffset (Variables|Default|GetDefaultSceneRoot) (Math|Vector|MakeVector 0.0 0.0 1.0) false false)
        (Variables|Default|SetCompteur_de_joueur 0)))))

(fn ConstructionScript
  (bind _new_mesh (Variables|Default|GetNew%20Mesh))
  (bind _new_mesh_2 (Variables|Default|GetNew%20Mesh))
  (bind _scaleplatform (Variables|Default|GetScalePlatform))
  (bind _returnvalue (StaticMesh|GetBoundingBox _new_mesh))
  (bind _returnvalue_2 (StaticMesh|GetBoundingBox _new_mesh_2))
  (bind _z (Math|Vector|BreakVector _scaleplatform))
  (bind _returnvalue_3 (- (.max _returnvalue_2) (.min _returnvalue_2)))
  (bind _returnvalue_4 (* (.z _returnvalue_3) _z))
  (Components|StaticMesh|SetStaticMesh (Variables|Default|GetMesh) (Variables|Default|GetNew%20Mesh))
  (Rendering|Material|SetMaterial (Variables|Default|GetMesh) 0 (Variables|Default|GetMaterial))
  (Transformation|SetWorldScale3D (Variables|Default|GetMesh) (Variables|Default|GetScalePlatform))
  (Transformation|SetWorldScale3D (Variables|Default|GetTrigerPhysics) (Variables|Default|GetScaleTrigger))
  (Transformation|SetRelativeLocation (Variables|Default|GetMesh) (Math|Vector|MakeVector 0.0 0.0 (/ (* (.z (- (.max _returnvalue) (.min _returnvalue))) (.z (Variables|Default|GetScalePlatform))) 2.0)) false false)
  (Transformation|SetRelativeLocation (Variables|Default|GetTrigerPhysics) (Math|Vector|MakeVector 0.0 0.0 (- (+ (.Z (Math|Vector|BreakVector (Components|Box|GetScaledBoxExtent (Variables|Default|GetTrigerPhysics)))) _returnvalue_4) _returnvalue_4)) false false))