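; Sliding platform that travels between its starting location and a TargetPoint when enough players step into its trigger.
; Overlaps of PlayerCapsule-tagged components are counted; reaching PlayerToSlide starts the outbound or return timeline, whichever end it rests at.
; Each timeline lerps the actor's location at its own play rate, and new moves are blocked while one plays.
; The construction script applies the configurable mesh and material, then scales and raises the trigger using the mesh's height.
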(event OnComponentBeginOverlap(Trigger)
  (params (OverlappedComponent :type Primitive%20Component%20Object%20Reference) (OtherActor :type Actor%20Object%20Reference) (OtherComp :type Primitive%20Component%20Object%20Reference) (OtherBodyIndex :type Integer) (bFromSweep :type Boolean) (SweepResult :type Hit%20Result%20Structure%20%28by%20ref%29))
  (if (Components|ComponentHasTag OtherComp "PlayerCapsule")
    (Variables|Default|SetPlayer%20cont (+ (Variables|Default|GetPlayer%20cont) 1))
    (if (>= (Variables|Default|GetPlayer%20cont) (Variables|Default|GetPlayerToSlide))
      (if (not (Variables|Default|GetIplayingTL))
        (if (Variables|Default|GetIsInDasePose)
          ;[0.15 0.15 0.15 0.5] TL
          (Components|Timeline|SetPlayRate (Variables|Default|GetTL_Aller) (Variables|TL|GetAllerRate))
          (bind _alfa (Timeline|TL_Aller PlayFromStart)
            (:Update
              (Transformation|SetActorLocation (Math|Vector|Lerp(Vector) (Variables|TL|GetBase%20pose) (Transformation|GetActorLocation (Variables|TL|GetTarget%20Point)) _alfa) false false)
              (Variables|Default|SetIplayingTL true))
            (:Finished
              (Variables|Default|SetIsInDasePose false)
              (Variables|Default|SetIplayingTL false)))
          (else
            (Components|Timeline|SetPlayRate (Variables|Default|GetTL_Retour) (Variables|TL|GetRetourRate))
            (bind _alfa_2 (Timeline|TL_Retour PlayFromStart)
              (:Update
                (Transformation|SetActorLocation (Math|Vector|Lerp(Vector) (Transformation|GetActorLocation (Variables|TL|GetTarget%20Point)) (Variables|TL|GetBase%20pose) _alfa_2) false false)
                (Variables|Default|SetIplayingTL true))
              (:Finished
                (Variables|Default|SetIsInDasePose true)
                (Variables|Default|SetIplayingTL false)))))))))

(event OnComponentEndOverlap(Trigger)
  (params (OverlappedComponent :type Primitive%20Component%20Object%20Reference) (OtherActor :type Actor%20Object%20Reference) (OtherComp :type Primitive%20Component%20Object%20Reference) (OtherBodyIndex :type Integer))
  (if (Components|ComponentHasTag OtherComp "PlayerCapsule")
    (Variables|Default|SetPlayer%20cont (- (Variables|Default|GetPlayer%20cont) 1))))

(event EventBeginPlay
  (Variables|TL|SetBase%20pose (Transformation|GetActorLocation)))

(event Collision|EventActorBeginOverlap
  (params (OtherActor :type Actor%20Object%20Reference)))

(event EventTick
  (params (DeltaSeconds :type Float%20%28single-precision%29)))

(fn ConstructionScript
  (bind _new_mesh (Variables|Default|GetNew%20Mesh))
  (bind _returnvalue (StaticMesh|GetBoundingBox _new_mesh))
  ;[0.15 0.15 0.15 0.5] Mesh
  (Components|StaticMesh|SetStaticMesh (Variables|Default|GetStaticMesh) (Variables|Default|GetNew%20Mesh))
  (Rendering|Material|SetMaterial (Variables|Default|GetStaticMesh) 0 (Variables|Default|GetMaterial))
  ;[0.15 0.15 0.15 0.5] Trigger
  (Transformation|SetWorldScale3D (Variables|Default|GetTrigger) (Variables|Default|GetScale%20trigger))
  (Transformation|SetRelativeLocation (Variables|Default|GetTrigger) (Math|Vector|MakeVector 0.0 0.0 (+ (.Z (Math|Vector|BreakVector (* (- (.max _returnvalue) (.min _returnvalue)) (Transformation|GetWorldScale (Variables|Default|GetStaticMesh))))) (.Z (Math|Vector|BreakVector (Components|Box|GetScaledBoxExtent (Variables|Default|GetTrigger)))))) false false))