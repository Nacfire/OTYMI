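; BP_DVD_Case is a DVD case prop whose appearance is set in the Construction Script, with no active event logic.
; It applies ScaleCase to both case meshes and shrinks the shake, home-in and destroy spheres to zero scale.
; CaseIsClosed swaps the first mesh to the closed model.
; The open-case setup, with two meshes and a lid offset, is present but never runs.
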(event EventBeginPlay)

(event Collision|EventActorBeginOverlap
  (params (OtherActor :type Actor%20Object%20Reference)))

(event EventTick
  (params (DeltaSeconds :type Float%20%28single-precision%29)))

(fn ConstructionScript
  (Transformation|SetWorldScale3D (Variables|Default|GetCase_1) (Variables|Default|GetScale_Case))
  (Transformation|SetWorldScale3D (Variables|Default|GetCase_2) (Variables|Default|GetScale_Case))
  (Transformation|SetWorldScale3D (Variables|Default|GetSphere_Shake) "0, 0, 0")
  (Transformation|SetWorldScale3D (Variables|Default|GetSphere_HomeIn) "0, 0, 0")
  (Transformation|SetWorldScale3D (Variables|Default|GetSphere_Destroy) "0, 0, 0")
  (if (Variables|Default|GetCaseIsClosed)
    (Components|StaticMesh|SetStaticMesh (Variables|Default|GetCase_1) (Variables|Default|GetMesh_Closed))))