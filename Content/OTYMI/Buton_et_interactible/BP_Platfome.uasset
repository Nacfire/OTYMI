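; One-way platform actor that lets the player drop down or jump up through it by toggling its mesh collision.
; Top and bottom trigger boxes react to "PlayerCapsule", cast the overlapping actor to BP_ThirdPersonPlayerController and poll held keys only when overlap begins.
; Matching input disables mesh collision, and leaving either box restores it.
; The construction script applies mesh, scale and a collision object type chosen by CableCanOverlap.
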(event OnComponentBeginOverlap(BoxTop)
  (params (OverlappedComponent :type Primitive%20Component%20Object%20Reference) (OtherActor :type Actor%20Object%20Reference) (OtherComp :type Primitive%20Component%20Object%20Reference) (OtherBodyIndex :type Integer) (bFromSweep :type Boolean) (SweepResult :type Hit%20Result%20Structure%20%28by%20ref%29))
  (if (Components|ComponentHasTag OtherComp "PlayerCapsule")
    (bind _asbp_third_person_player_controller (Utilities|Casting|CastToBP_ThirdPersonPlayerController OtherActor))
    (if (or (and (> (Class|PlayerController|GetInputKeyTimeDown _asbp_third_person_player_controller "Down") 0.0) (> (Class|PlayerController|GetInputKeyTimeDown _asbp_third_person_player_controller "Up") 0.0)) (and (> (Class|PlayerController|GetInputKeyTimeDown _asbp_third_person_player_controller "Gamepad_LeftY") 0.0) (> (Class|PlayerController|GetInputKeyTimeDown _asbp_third_person_player_controller "Gamepad_FaceButton_Bottom") 0.0)))
      (Collision|SetCollisionEnabled (Variables|Default|GetMesh) "NoCollision"))))

(event OnComponentBeginOverlap(BoxDown)
  (params (OverlappedComponent :type Primitive%20Component%20Object%20Reference) (OtherActor :type Actor%20Object%20Reference) (OtherComp :type Primitive%20Component%20Object%20Reference) (OtherBodyIndex :type Integer) (bFromSweep :type Boolean) (SweepResult :type Hit%20Result%20Structure%20%28by%20ref%29))
  (if (Components|ComponentHasTag OtherComp "PlayerCapsule")
    (bind _asbp_third_person_player_controller (Utilities|Casting|CastToBP_ThirdPersonPlayerController OtherActor))
    (if (or (> (Class|PlayerController|GetInputKeyTimeDown _asbp_third_person_player_controller "Up") 0.0) (> (Class|PlayerController|GetInputKeyTimeDown _asbp_third_person_player_controller "Gamepad_FaceButton_Bottom") 0.0))
      (Collision|SetCollisionEnabled (Variables|Default|GetMesh) "NoCollision"))))

(event OnComponentEndOverlap(BoxTop)
  (params (OverlappedComponent :type Primitive%20Component%20Object%20Reference) (OtherActor :type Actor%20Object%20Reference) (OtherComp :type Primitive%20Component%20Object%20Reference) (OtherBodyIndex :type Integer))
  (if (Components|ComponentHasTag OtherComp "PlayerCapsule")
    (Collision|SetCollisionEnabled (Variables|Default|GetMesh) "QueryAndPhysics")))

(event OnComponentEndOverlap(BoxDown)
  (params (OverlappedComponent :type Primitive%20Component%20Object%20Reference) (OtherActor :type Actor%20Object%20Reference) (OtherComp :type Primitive%20Component%20Object%20Reference) (OtherBodyIndex :type Integer))
  (if (Components|ComponentHasTag OtherComp "PlayerCapsule")
    (Collision|SetCollisionEnabled (Variables|Default|GetMesh) "QueryAndPhysics")))

(event EventBeginPlay)

(event Collision|EventActorBeginOverlap
  (params (OtherActor :type Actor%20Object%20Reference)))

(event EventTick
  (params (DeltaSeconds :type Float%20%28single-precision%29)))

(fn ConstructionScript
  (Components|StaticMesh|SetStaticMesh (Variables|Default|GetMesh) (Variables|Default|GetStatic_Mesh))
  (Transformation|SetWorldScale3D (Variables|Default|GetMesh) (Variables|Default|GetScale))
  (if (Variables|Default|GetCable_Can_Overlap)
    (Collision|SetCollisionObjectType (Variables|Default|GetMesh) "ECC_GameTraceChannel1")
    (else
      (Collision|SetCollisionObjectType (Variables|Default|GetMesh) "ECC_WorldDynamic"))))