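; Sliding door actor that moves its mesh between its origin and FinalLocation through Open and Close events.
; When Coulise is set, each event plays a timeline that lerps the relative location, with play rate derived from TLOpenRate in both directions.
; Timelines update IsPlayingTL and IsOpen, and IsOpen gates both events.
; The construction script applies the configurable static mesh and scale.
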(event EventBeginPlay)

(event Collision|EventActorBeginOverlap
  (params (OtherActor :type Actor%20Object%20Reference)))

(event EventTick
  (params (DeltaSeconds :type Float%20%28single-precision%29)))

(event EventOpen
  (if (not (Variables|Default|GetIs%20open))
    (if (Variables|Default|GetCoulise)
      (Components|Timeline|SetPlayRate (Variables|Default|GetTL_Open) (/ 1.0 (Variables|Porte_coulisante|GetTL_OpenRate)))
      (bind _open_close (Timeline|TL_Open PlayFromStart)
        (:Update
          (Transformation|SetRelativeLocationAndRotation (Variables|Default|GetMesh) (Math|Vector|Lerp(Vector) "0, 0, 0" (Variables|Porte_coulisante|GetFinal_Location) _open_close) "0, 0, 0" false false)
          (Variables|Default|SetIsPlayingTL true))
        (:Finished
          (Variables|Default|SetIsPlayingTL false)
          (Variables|Default|SetIs%20open true))))))

(event EventClose
  (if (Variables|Default|GetIs%20open)
    (if (Variables|Default|GetCoulise)
      (Components|Timeline|SetPlayRate (Variables|Default|GetTLClose) (/ 1.0 (Variables|Porte_coulisante|GetTL_OpenRate)))
      (bind _open_close (Timeline|TLClose PlayFromStart)
        (:Update
          (Transformation|SetRelativeLocationAndRotation (Variables|Default|GetMesh) (Math|Vector|Lerp(Vector) (Variables|Porte_coulisante|GetFinal_Location) "0, 0, 0" _open_close) "0, 0, 0" false false)
          (Variables|Default|SetIsPlayingTL true))
        (:Finished
          (Variables|Default|SetIsPlayingTL false)
          (Variables|Default|SetIs%20open false))))))

(fn ConstructionScript
  (Components|StaticMesh|SetStaticMesh (Variables|Default|GetMesh) (Variables|Default|GetStatic_mesh))
  (Transformation|SetWorldScale3D (Variables|Default|GetMesh) (Variables|Default|GetScale)))