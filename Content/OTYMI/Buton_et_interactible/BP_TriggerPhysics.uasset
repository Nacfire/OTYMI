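; BP_TriggerPhysics is a one-shot trigger volume that turns on physics for its assigned interactibles when the player capsule enters, after a short delay.
; If DestoyAferGetPhysique is set, a fast looping timer freezes each one whose velocity nears zero, removes it from the working array, and pauses once that array is empty.
; The construction script sizes the trigger and copies ArrayInteractible into that working array.
; An unconnected CanPhysics-tag branch for BP_Platform-fall never runs.
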(event OnComponentBeginOverlap(Trigger)
  (params (OverlappedComponent :type Primitive%20Component%20Object%20Reference) (OtherActor :type Actor%20Object%20Reference) (OtherComp :type Primitive%20Component%20Object%20Reference) (OtherBodyIndex :type Integer) (bFromSweep :type Boolean) (SweepResult :type Hit%20Result%20Structure%20%28by%20ref%29))
  (if (Components|ComponentHasTag OtherComp "PlayerCapsule")
    (if (not (Variables|Default|GetActivate))
      (Utilities|FlowControl|Delay 0.2)
      (Variables|Default|SetActivate true)
      (for _array_element (Variables|Default|GetArrayInteractibleCode)
        (Variables|Default|SetInteractible _array_element)
        (Physics|SetSimulatePhysics (Variables|/Game/OTYMI/Buton_et_interactible/BP_Platform-fall.BP_Platform-fall_C|GetMesh (Variables|Default|GetInteractible)) true))
      (Development|PrintString "Physics")
      (if (Variables|Default|GetDestoy%20afer%20Get%20physique)
        (if (Utilities|Time|IsValidTimerHandle (Variables|Default|GetTimerRef))
          (Utilities|Time|UnpauseTimerbyHandle (Variables|Default|GetTimerRef))
          (else
            (bind _returnvalue (Utilities|Time|SetTimerbyEvent (delegate Custom|Check%20velocity%20Ref) 0.01 true))
            (Variables|Default|SetTimerRef _returnvalue)))))))

(event Custom|Check%20velocity%20Ref
  (for _array_element (Variables|Default|GetArrayInteractibleCode)
    (Variables|Default|SetInteractible _array_element)
    (if (Utilities|Operators|EqualEqual :A (Transformation|GetVelocity (Variables|Default|GetInteractible)) :ErrorTolerance 1.0)
      (Physics|SetSimulatePhysics (Variables|/Game/OTYMI/Buton_et_interactible/BP_Platform-fall.BP_Platform-fall_C|GetMesh (Variables|Default|GetInteractible)) false)
      (Utilities|Array|RemoveItem (Variables|Default|GetArrayInteractibleCode) (Variables|Default|GetInteractible))
      (Development|PrintString "Stop physics")))
  (if (Utilities|Array|IsEmpty (Variables|Default|GetArrayInteractibleCode))
    (Utilities|Time|PauseTimerbyHandle (Variables|Default|GetTimerRef))))

(event EventBeginPlay)

(event Collision|EventActorBeginOverlap
  (params (OtherActor :type Actor%20Object%20Reference)))

(event EventTick
  (params (DeltaSeconds :type Float%20%28single-precision%29)))

(fn ConstructionScript
  (Utilities|Array|Clear (Variables|Default|GetArrayInteractibleCode))
  (Transformation|SetWorldScale3D (Variables|Default|GetTrigger) (Variables|Default|GetScaleTrigger))
  (for _array_element (Variables|Default|GetArrayInteractible)
    (Utilities|Array|Add (Variables|Default|GetArrayInteractibleCode) _array_element)))