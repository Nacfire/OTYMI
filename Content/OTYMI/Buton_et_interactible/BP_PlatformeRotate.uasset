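; Rotating platform actor that swings between its placed rotation and a target rotation, either once or in a continuous loop.
; The construction script applies the configurable mesh, material and scale, and stores the starting rotation.
; Open and Close share a one-shot Activate guard, then run delayed timelines with adjustable rates that lerp the root's world rotation.
; With Loop enabled, each finished timeline starts the opposite one.
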(event Custom|PlayStartOpen
  (Components|Timeline|SetPlayRate (Variables|Default|GetTL_Open) (/ 1.0 (Variables|PlatfomPivot|GetTL_OpenRate)))
  (Variables|Default|SetIsPlayingTL true)
  (Utilities|FlowControl|Delay (Variables|PlatfomPivot|GetWaitBeforeOpen))
  (bind _open_close (Timeline|TL_Open PlayFromStart)
    (:Update
      (Transformation|SetWorldRotation (Variables|Default|GetDefaultSceneRoot) (Math|Rotator|Lerp(Rotator) (Variables|PlatfomPivot|GetBase%20Rotation) (Variables|PlatfomPivot|GetFinal_Rotation) _open_close) false false))
    (:Finished
      (Variables|Default|SetIsPlayingTL false)
      (Variables|Default|SetIs%20open true)
      (if (Variables|PlatfomPivot|GetLoop)
        (CallFunction|PlayStartClose)))))

(event Custom|PlayStartClose
  (Components|Timeline|SetPlayRate (Variables|Default|GetTLClose) (/ 1.0 (Variables|PlatfomPivot|GetTL_CloseRate)))
  (Variables|Default|SetIsPlayingTL true)
  (Utilities|FlowControl|Delay (Variables|PlatfomPivot|GetWaitBeforeClose))
  (bind _open_close (Timeline|TLClose PlayFromStart)
    (:Update
      (Transformation|SetWorldRotation (Variables|Default|GetDefaultSceneRoot) (Math|Rotator|Lerp(Rotator) (Variables|PlatfomPivot|GetFinal_Rotation) (Variables|PlatfomPivot|GetBase%20Rotation) _open_close) false false))
    (:Finished
      (Variables|Default|SetIsPlayingTL false)
      (Variables|Default|SetIs%20open false)
      (if (Variables|PlatfomPivot|GetLoop)
        (CallFunction|PlayStartOpen)))))

(event EventBeginPlay)

(event Collision|EventActorBeginOverlap
  (params (OtherActor :type Actor%20Object%20Reference)))

(event EventTick
  (params (DeltaSeconds :type Float%20%28single-precision%29)))

(event EventOpen
  (if (not (Variables|Default|GetActivate))
    (Variables|Default|SetActivate true)
    (if (not (Variables|Default|GetIs%20open))
      (Components|Timeline|SetPlayRate (Variables|Default|GetTL_Open) (/ 1.0 (Variables|PlatfomPivot|GetTL_OpenRate)))
      (Variables|Default|SetIsPlayingTL true)
      (Utilities|FlowControl|Delay (Variables|PlatfomPivot|GetWaitBeforeOpen))
      (bind _open_close (Timeline|TL_Open PlayFromStart)
        (:Update
          (Transformation|SetWorldRotation (Variables|Default|GetDefaultSceneRoot) (Math|Rotator|Lerp(Rotator) (Variables|PlatfomPivot|GetBase%20Rotation) (Variables|PlatfomPivot|GetFinal_Rotation) _open_close) false false))
        (:Finished
          (Variables|Default|SetIsPlayingTL false)
          (Variables|Default|SetIs%20open true)
          (if (Variables|PlatfomPivot|GetLoop)
            (CallFunction|PlayStartClose)))))))

(event EventClose
  (if (not (Variables|Default|GetActivate))
    (Variables|Default|SetActivate true)
    (if (Variables|Default|GetIs%20open)
      (Components|Timeline|SetPlayRate (Variables|Default|GetTLClose) (/ 1.0 (Variables|PlatfomPivot|GetTL_CloseRate)))
      (Variables|Default|SetIsPlayingTL true)
      (Utilities|FlowControl|Delay (Variables|PlatfomPivot|GetWaitBeforeClose))
      (bind _open_close (Timeline|TLClose PlayFromStart)
        (:Update
          (Transformation|SetWorldRotation (Variables|Default|GetDefaultSceneRoot) (Math|Rotator|Lerp(Rotator) (Variables|PlatfomPivot|GetFinal_Rotation) (Variables|PlatfomPivot|GetBase%20Rotation) _open_close) false false))
        (:Finished
          (Variables|Default|SetIsPlayingTL false)
          (Variables|Default|SetIs%20open false)
          (if (Variables|PlatfomPivot|GetLoop)
            (CallFunction|PlayStartOpen)))))))

(fn ConstructionScript
  (Components|StaticMesh|SetStaticMesh (Variables|Default|GetMesh) (Variables|Default|GetStatic_mesh))
  (Rendering|Material|SetMaterial (Variables|Default|GetMesh) 0 (Variables|Default|GetMaterial))
  (Transformation|SetWorldScale3D (Variables|Default|GetMesh) (Variables|Default|GetScale))
  (Variables|PlatfomPivot|SetBase%20Rotation (Transformation|GetWorldRotation (Variables|Default|GetDefaultSceneRoot))))