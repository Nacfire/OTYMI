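; Seesaw actor that tilts when enough player capsules stand on its left or right end.
; Two triggers count tagged overlaps against per-side thresholds, setting turn flags and starting a looping timer.
; Each timer tick steps pitch toward a side's limit or back to the BeginPlay pose, pausing when no step applies.
; The construction script applies the configurable mesh and material, then scales and positions both triggers from the mesh bounds.
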(event OnComponentBeginOverlap(RightTrigger)
  (params (OverlappedComponent :type Primitive%20Component%20Object%20Reference) (OtherActor :type Actor%20Object%20Reference) (OtherComp :type Primitive%20Component%20Object%20Reference) (OtherBodyIndex :type Integer) (bFromSweep :type Boolean) (SweepResult :type Hit%20Result%20Structure%20%28by%20ref%29))
  (if (Components|ComponentHasTag OtherComp "PlayerCapsule")
    (Variables|Right|SetRight_PlayerCont (+ (Variables|Right|GetRight_PlayerCont) 1))
    (if (>= (Variables|Right|GetRight_PlayerCont) (Variables|Right|GetNeedPlayerToTurnRight))
      (Variables|Right|SetTurnRight true)
      (CallFunction|StartMove))))

(event OnComponentEndOverlap(RightTrigger)
  (params (OverlappedComponent :type Primitive%20Component%20Object%20Reference) (OtherActor :type Actor%20Object%20Reference) (OtherComp :type Primitive%20Component%20Object%20Reference) (OtherBodyIndex :type Integer))
  (if (Components|ComponentHasTag OtherComp "PlayerCapsule")
    (Variables|Right|SetRight_PlayerCont (- (Variables|Right|GetRight_PlayerCont) 1))
    (if (< (Variables|Right|GetRight_PlayerCont) (Variables|Right|GetNeedPlayerToTurnRight))
      (Variables|Right|SetTurnRight false))))

(event OnComponentBeginOverlap(LeftTrigger)
  (params (OverlappedComponent :type Primitive%20Component%20Object%20Reference) (OtherActor :type Actor%20Object%20Reference) (OtherComp :type Primitive%20Component%20Object%20Reference) (OtherBodyIndex :type Integer) (bFromSweep :type Boolean) (SweepResult :type Hit%20Result%20Structure%20%28by%20ref%29))
  (if (Components|ComponentHasTag OtherComp "PlayerCapsule")
    (Variables|Left|SetLeft_PlayerCont (+ (Variables|Left|GetLeft_PlayerCont) 1))
    (if (>= (Variables|Left|GetLeft_PlayerCont) (Variables|Left|GetNeedPlayerToTurnLeft))
      (Variables|Left|SetTurnLeft true)
      (CallFunction|StartMove))))

(event OnComponentEndOverlap(LeftTrigger)
  (params (OverlappedComponent :type Primitive%20Component%20Object%20Reference) (OtherActor :type Actor%20Object%20Reference) (OtherComp :type Primitive%20Component%20Object%20Reference) (OtherBodyIndex :type Integer))
  (if (Components|ComponentHasTag OtherComp "PlayerCapsule")
    (Variables|Left|SetLeft_PlayerCont (- (Variables|Left|GetLeft_PlayerCont) 1))
    (if (< (Variables|Left|GetLeft_PlayerCont) (Variables|Left|GetNeedPlayerToTurnLeft))
      (Variables|Left|SetTurnLeft false))))

(event Custom|StartMove
  (if (Utilities|Time|IsValidTimerHandle (Variables|Default|GetTimer))
    (Utilities|Time|UnpauseTimerbyHandle (Variables|Default|GetTimer))
    (else
      (bind _returnvalue (Utilities|Time|SetTimerbyEvent (delegate Custom|Move) 0.01 true))
      (Variables|Default|SetTimer _returnvalue))))

(event Custom|Move
  (bind _returnvalue (Transformation|GetActorRotation))
  (bind _returnvalue_2 (Transformation|GetActorRotation))
  (bind _returnvalue_3 (Transformation|GetActorRotation))
  (bind _returnvalue_4 (Transformation|GetActorRotation))
  (bind _returnvalue_5 (Transformation|GetActorRotation))
  (bind _returnvalue_6 (Transformation|GetActorRotation))
  (if (and (not (Utilities|Operators|EqualEqual (Transformation|GetActorRotation) (Variables|Left|GetMax%20Left%20RotateY) 0.1)) (Variables|Left|GetTurnLeft))
    (Transformation|SetActorRotation (Math|Rotator|MakeRotator (.roll _returnvalue_6) (+ (.pitch _returnvalue_6) (Variables|Move|GetSpeed)) (.yaw _returnvalue_6)))
    (elif (and (not (Utilities|Operators|EqualEqual (Transformation|GetActorRotation) (Variables|Move|GetBase%20pose) 0.1)) (not (Variables|Right|GetTurnRight)))
      (if (>= (.pitch (Transformation|GetActorRotation)) (.pitch (Variables|Move|GetBase%20pose)))
        (Transformation|SetActorRotation (Math|Rotator|MakeRotator (.roll _returnvalue_2) (- (.pitch _returnvalue_2) (Variables|Move|GetSpeed)) (.yaw _returnvalue_2)))
        (else
          (Transformation|SetActorRotation (Math|Rotator|MakeRotator (.roll _returnvalue_4) (+ (.pitch _returnvalue_4) (Variables|Move|GetSpeed)) (.yaw _returnvalue_4)))))
      (elif (and (not (Utilities|Operators|EqualEqual (Transformation|GetActorRotation) (Variables|Right|GetMax%20Right%20RotateY) 0.1)) (Variables|Right|GetTurnRight))
        (Transformation|SetActorRotation (Math|Rotator|MakeRotator (.roll _returnvalue) (- (.pitch _returnvalue) (Variables|Move|GetSpeed)) (.yaw _returnvalue)))
        (elif (and (not (Utilities|Operators|EqualEqual (Transformation|GetActorRotation) (Variables|Move|GetBase%20pose) 0.1)) (not (Variables|Left|GetTurnLeft)))
          (if (>= (.pitch (Transformation|GetActorRotation)) (.pitch (Variables|Move|GetBase%20pose)))
            (Transformation|SetActorRotation (Math|Rotator|MakeRotator (.roll _returnvalue_5) (+ (.pitch _returnvalue_5) (Variables|Move|GetSpeed)) (.yaw _returnvalue_5)))
            (else
              (Transformation|SetActorRotation (Math|Rotator|MakeRotator (.roll _returnvalue_3) (- (.pitch _returnvalue_3) (Variables|Move|GetSpeed)) (.yaw _returnvalue_3)))))
          (else
            (Utilities|Time|PauseTimerbyHandle (Variables|Default|GetTimer))))))))

(event EventBeginPlay
  (Variables|Move|SetBase%20pose (Transformation|GetActorRotation)))

(event Collision|EventActorBeginOverlap
  (params (OtherActor :type Actor%20Object%20Reference)))

(event EventTick
  (params (DeltaSeconds :type Float%20%28single-precision%29)))

(fn ConstructionScript
  (bind _staticmesh (Variables|Default|GetStaticMesh))
  (bind _new_mesh (Variables|Default|GetNew%20Mesh))
  (bind _new_mesh_2 (Variables|Default|GetNew%20Mesh))
  (bind _staticmesh_2 (Variables|Default|GetStaticMesh))
  (bind _returnvalue (StaticMesh|GetBoundingBox _new_mesh_2))
  (bind _returnvalue_2 (Transformation|GetWorldScale _staticmesh))
  (bind _returnvalue_3 (StaticMesh|GetBoundingBox _new_mesh))
  (bind _returnvalue_4 (Transformation|GetWorldScale _staticmesh_2))
  (bind _returnvalue_5 (- (.max _returnvalue) (.min _returnvalue)))
  (bind _returnvalue_6 (- (.max _returnvalue_3) (.min _returnvalue_3)))
  (bind _returnvalue_7 (* _returnvalue_5 _returnvalue_4))
  (bind _returnvalue_8 (* _returnvalue_6 _returnvalue_2))
  (bind (_x _y _z) (Math|Vector|BreakVector _returnvalue_8))
  (bind (_x_2 _y_2 _z_2) (Math|Vector|BreakVector _returnvalue_7))
  (Components|StaticMesh|SetStaticMesh (Variables|Default|GetStaticMesh) (Variables|Default|GetNew%20Mesh))
  (Rendering|Material|SetMaterial (Variables|Default|GetStaticMesh) 0 (Variables|Default|GetMaterial))
  ;[0.15 0.15 0.15 0.5] Left Trigger
  (Transformation|SetWorldScale3D (Variables|Default|GetLeftTrigger) (Variables|Default|GetScale_LeftTrigger))
  (Transformation|SetRelativeLocation (Variables|Default|GetLeftTrigger) (Math|Vector|MakeVector (/ (- (/ _x (Variables|Left|GetOffsetLeft%28proportion%29)) (/ _x 2.0)) (.X (Math|Vector|BreakVector (Transformation|GetWorldScale (Variables|Default|GetStaticMesh))))) 0.0 _z) false false)
  ;[0.15 0.15 0.15 0.5] Left Trigger
  (Transformation|SetWorldScale3D (Variables|Default|GetRightTrigger) (Variables|Default|GetScale_RightTrigger))
  (Transformation|SetRelativeLocation (Variables|Default|GetRightTrigger) (Math|Vector|MakeVector (/ (- (/ _x_2 2.0) (/ _x_2 (Variables|Right|GetOffsetRight%28Proportion%29))) (.X (Math|Vector|BreakVector (Transformation|GetWorldScale (Variables|Default|GetStaticMesh))))) 0.0 _z_2) false false))