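; BP_PlatformFall is a configurable platform actor whose name suggests a falling platform, though the graphs shown contain no fall logic.
; The Construction Script applies variables for static mesh, material, world scale and mass override to the Mesh component, so each instance can differ in look and weight.
; The Event Graph holds only disabled placeholder events, so any falling behavior depends on settings outside these graphs.
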(event EventBeginPlay)

(event Collision|EventActorBeginOverlap
  (params (OtherActor :type Actor%20Object%20Reference)))

(event EventTick
  (params (DeltaSeconds :type Float%20%28single-precision%29)))

(fn ConstructionScript
  (Components|StaticMesh|SetStaticMesh (Variables|Default|GetMesh) (Variables|Default|GetNew%20Mesh))
  (Rendering|Material|SetMaterial (Variables|Default|GetMesh) 0 (Variables|Default|GetMaterial))
  (Transformation|SetWorldScale3D (Variables|Default|GetMesh) (Variables|Default|GetScale))
  (Class|PrimitiveComponent|SetMassOverrideinKg (Variables|Default|GetMesh) "None" (Variables|Default|GetMass%20in%20Kg) true))