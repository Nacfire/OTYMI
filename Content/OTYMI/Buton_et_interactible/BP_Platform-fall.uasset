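; BP_Platform-fall is a platform that starts physics simulation when triggered and freezes again once it comes to rest.
; Its Box trigger enables physics on an overlapping BP_Platform-fall tagged CanPhysics, or on itself when UseTriggerByPlayer is set and the player capsule enters.
; A looping timer polls the moving mesh's velocity, disabling simulation and pausing itself near zero.
; The construction script applies mesh, material, scale and mass, and sits the trigger above the mesh.
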(event OnComponentBeginOverlap(Box)
  (params (OverlappedComponent :type Primitive%20Component%20Object%20Reference) (OtherActor :type Actor%20Object%20Reference) (OtherComp :type Primitive%20Component%20Object%20Reference) (OtherBodyIndex :type Integer) (bFromSweep :type Boolean) (SweepResult :type Hit%20Result%20Structure%20%28by%20ref%29))
  (bind _asbp_platform_fall (Utilities|Casting|CastToBP_Platform-fall OtherActor))
  (if (Actor|ActorHasTag OtherActor "CanPhysics")
    (Physics|SetSimulatePhysics (Variables|BP_Platform-fall_C|GetMesh _asbp_platform_fall) true)
    (Variables|Default|SetInteractible _asbp_platform_fall)
    (if (Utilities|Time|IsValidTimerHandle (Variables|Default|GetTimerRef)) :!label _label
      (Utilities|Time|UnpauseTimerbyHandle (Variables|Default|GetTimerRef))
      (else
        (bind _returnvalue (Utilities|Time|SetTimerbyEvent (delegate Custom|Check%20velocity%20Ref) 0.1 true))
        (Variables|Default|SetTimerRef _returnvalue)))
    (elif (Variables|Default|GetUse%20Trigger%20By%20Player)
      (if (Components|ComponentHasTag OtherComp "PlayerCapsule")
        (Variables|Default|SetInteractible self)
        (Physics|SetSimulatePhysics (Variables|BP_Platform-fall_C|GetMesh (Variables|Default|GetInteractible)) true)
        (goto _label)))))

(event Custom|Check%20velocity%20Ref
  (if (Utilities|Operators|EqualEqual :A (Transformation|GetComponentVelocity (Variables|BP_Platform-fall_C|GetMesh (Variables|Default|GetInteractible))) :ErrorTolerance 1.0)
    (Physics|SetSimulatePhysics (Variables|BP_Platform-fall_C|GetMesh (Variables|Default|GetInteractible)) false)
    (Utilities|Time|PauseTimerbyHandle (Variables|Default|GetTimerRef))))

(event EventBeginPlay)

(event Collision|EventActorBeginOverlap
  (params (OtherActor :type Actor%20Object%20Reference)))

(event EventTick
  (params (DeltaSeconds :type Float%20%28single-precision%29)))

(fn ConstructionScript
  (Components|StaticMesh|SetStaticMesh (Variables|Default|GetMesh) (Variables|Default|GetNew%20Mesh))
  (Rendering|Material|SetMaterial (Variables|Default|GetMesh) 0 (Variables|Default|GetMaterial))
  (Transformation|SetWorldScale3D (Variables|Default|GetMesh) (Variables|Default|GetScale))
  (Class|PrimitiveComponent|SetMassOverrideinKg (Variables|Default|GetMesh) "None" (Variables|Default|GetMass%20in%20Kg) true)
  (Transformation|SetWorldScale3D (Variables|Default|GetBox) (Variables|Default|GetScaleTrigger))
  (Transformation|SetWorldLocation (Variables|Default|GetBox) (+ (Transformation|GetWorldLocation (Variables|Default|GetMesh)) (Math|Vector|MakeVector 0.0 0.0 (.Z (Math|Vector|BreakVector (Components|Box|GetScaledBoxExtent (Variables|Default|GetBox)))))) false false))