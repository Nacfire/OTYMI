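; BP_Platfome1Way is a configurable one-way platform the player can jump up through from below.
; When the player capsule enters BoxDown while Up or the gamepad bottom face button is held, mesh collision turns off and the character is launched; leaving BoxDown restores collision.
; Construction applies mesh and scale and picks the collision object type from CableCanOverlap.
; The top-box drop-through logic is disconnected.
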(event OnComponentBeginOverlap(BoxTop)
  (params (OverlappedComponent :type Primitive%20Component%20Object%20Reference) (OtherActor :type Actor%20Object%20Reference) (OtherComp :type Primitive%20Component%20Object%20Reference) (OtherBodyIndex :type Integer) (bFromSweep :type Boolean) (SweepResult :type Hit%20Result%20Structure%20%28by%20ref%29)))

(event OnComponentBeginOverlap(BoxDown)
  (params (OverlappedComponent :type Primitive%20Component%20Object%20Reference) (OtherActor :type Actor%20Object%20Reference) (OtherComp :type Primitive%20Component%20Object%20Reference) (OtherBodyIndex :type Integer) (bFromSweep :type Boolean) (SweepResult :type Hit%20Result%20Structure%20%28by%20ref%29))
  (if (Variables|Default|GetJumpCanOverlap)
    (if (Components|ComponentHasTag OtherComp "PlayerCapsule")
      (bind _asbp_third_person_character (Utilities|Casting|CastToBP_ThirdPersonCharacter OtherActor))
      (if (or (> (Class|PlayerController|GetInputKeyTimeDown (Variables|/Game/ThirdPerson/Blueprints/BP_ThirdPersonCharacter.BP_ThirdPersonCharacter_C|GetPlayer%20Ref _asbp_third_person_character) "Up") 0.0) (> (Class|PlayerController|GetInputKeyTimeDown (Variables|/Game/ThirdPerson/Blueprints/BP_ThirdPersonCharacter.BP_ThirdPersonCharacter_C|GetPlayer%20Ref _asbp_third_person_character) "Gamepad_FaceButton_Bottom") 0.0))
        (Collision|SetCollisionEnabled (Variables|Default|GetMesh) "NoCollision")
        (bind _ascharacter (Utilities|Casting|CastToCharacter OtherActor))
        (Character|LaunchCharacter _ascharacter (Variables|Default|GetLaunch%20Velocity) false false)))))

(event OnComponentEndOverlap(BoxTop)
  (params (OverlappedComponent :type Primitive%20Component%20Object%20Reference) (OtherActor :type Actor%20Object%20Reference) (OtherComp :type Primitive%20Component%20Object%20Reference) (OtherBodyIndex :type Integer)))

(event OnComponentEndOverlap(BoxDown)
  (params (OverlappedComponent :type Primitive%20Component%20Object%20Reference) (OtherActor :type Actor%20Object%20Reference) (OtherComp :type Primitive%20Component%20Object%20Reference) (OtherBodyIndex :type Integer))
  (if (Components|ComponentHasTag OtherComp "PlayerCapsule")
    (Collision|SetCollisionEnabled (Variables|Default|GetMesh) "QueryAndPhysics")))

(event EventBeginPlay)

(event Collision|EventActorBeginOverlap
  (params (OtherActor :type Actor%20Object%20Reference)))

(event EventTick
  (params (DeltaSeconds :type Float%20%28single-precision%29)))

(fn ConstructionScript
  (Components|StaticMesh|SetStaticMesh (Variables|Default|GetMesh) (Variables|Default|GetStatic_Mesh))
  (Transformation|SetWorldScale3D (Variables|Default|GetMesh) (Variables|Default|GetScale))
  (if (Variables|Default|GetCable_Can_Overlap)
    (Collision|SetCollisionObjectType (Variables|Default|GetMesh) "ECC_GameTraceChannel2")
    (else
      (Collision|SetCollisionObjectType (Variables|Default|GetMesh) "ECC_WorldDynamic"))))