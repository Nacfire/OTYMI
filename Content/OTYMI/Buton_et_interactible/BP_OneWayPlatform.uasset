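; BP_OneWayPlatform is a one-way platform that is solid or passable separately for each of up to four players.
; When a BP_ThirdPersonCharacter's component tagged PlayerCapsule enters the Trigger, Platf blocks that player's collision channel, and leaving sets it back to Ignore.
; Each PlayerID maps to its own custom trace channel, so one player's overlap does not change the platform's response to the others.
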(event OnComponentBeginOverlap(Trigger)
  (params (OverlappedComponent :type Primitive%20Component%20Object%20Reference) (OtherActor :type Actor%20Object%20Reference) (OtherComp :type Primitive%20Component%20Object%20Reference) (OtherBodyIndex :type Integer) (bFromSweep :type Boolean) (SweepResult :type Hit%20Result%20Structure%20%28by%20ref%29))
  (if (Components|ComponentHasTag OtherComp "PlayerCapsule")
    (bind _asbp_third_person_character (Utilities|Casting|CastToBP_ThirdPersonCharacter OtherActor))
    (switch int (Variables|/Game/ThirdPerson/Blueprints/BP_ThirdPersonCharacter.BP_ThirdPersonCharacter_C|GetPlayerID _asbp_third_person_character)
      (:0
        (Variables|Default|SetChannel "ECC_GameTraceChannel1"))
      (:1
        (Variables|Default|SetChannel "ECC_GameTraceChannel3"))
      (:2
        (Variables|Default|SetChannel "ECC_GameTraceChannel4"))
      (:3
        (Variables|Default|SetChannel "ECC_GameTraceChannel5")))
    (Collision|SetCollisionResponsetoChannel (Variables|Default|GetPlatf) (Variables|Default|GetChannel) "ECR_Block")))

(event OnComponentEndOverlap(Trigger)
  (params (OverlappedComponent :type Primitive%20Component%20Object%20Reference) (OtherActor :type Actor%20Object%20Reference) (OtherComp :type Primitive%20Component%20Object%20Reference) (OtherBodyIndex :type Integer))
  (if (Components|ComponentHasTag OtherComp "PlayerCapsule")
    (bind _asbp_third_person_character (Utilities|Casting|CastToBP_ThirdPersonCharacter OtherActor))
    (switch int (Variables|/Game/ThirdPerson/Blueprints/BP_ThirdPersonCharacter.BP_ThirdPersonCharacter_C|GetPlayerID _asbp_third_person_character)
      (:0
        (Variables|Default|SetChannel "ECC_GameTraceChannel1"))
      (:1
        (Variables|Default|SetChannel "ECC_GameTraceChannel3"))
      (:2
        (Variables|Default|SetChannel "ECC_GameTraceChannel4"))
      (:3
        (Variables|Default|SetChannel "ECC_GameTraceChannel5")))
    (Collision|SetCollisionResponsetoChannel (Variables|Default|GetPlatf) (Variables|Default|GetChannel) "ECR_Ignore")))

(event EventBeginPlay)

(event Collision|EventActorBeginOverlap
  (params (OtherActor :type Actor%20Object%20Reference)))

(event EventTick
  (params (DeltaSeconds :type Float%20%28single-precision%29)))

(fn ConstructionScript)