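; BP_Roomba is a configurable Roomba actor whose graphs contain only construction-time setup, with no runtime logic.
; The construction script applies the exposed mesh, material and scale, then sizes a box and two detection-style spheres, the far one twice the close radius.
; It rests the box on the mesh origin and places the Eye light at a scale-adjusted offset with configurable pitch and cone width.
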(event EventTick
  (params (DeltaSeconds :type Float%20%28single-precision%29)))

(fn ConstructionScript
  (bind _scalesphere (Variables|Default|GetScaleSphere))
  (Components|StaticMesh|SetStaticMesh (Variables|Default|GetRoombaMesh) (Variables|Default|GetNewMesh))
  (Rendering|Material|SetMaterial (Variables|Default|GetRoombaMesh) 0 (Variables|Default|GetNewMat))
  (Transformation|SetWorldScale3D (Variables|Default|GetRoombaMesh) (Variables|Default|GetScaleMesh))
  (Components|Box|SetBoxExtent (Variables|Default|GetBox) (Variables|Default|GetScaleBox) true)
  (Components|Sphere|SetSphereRadius (Variables|Default|GetSphereClose) _scalesphere true)
  (Components|Sphere|SetSphereRadius (Variables|Default|GetSphereFar) (* _scalesphere 2.0) true)
  (Transformation|SetWorldLocation (Variables|Default|GetBox) (+ (Transformation|GetWorldLocation (Variables|Default|GetRoombaMesh)) (Math|Vector|MakeVector 0.0 0.0 (.Z (Math|Vector|BreakVector (Components|Box|GetScaledBoxExtent (Variables|Default|GetBox)))))) false false)
  (Transformation|SetWorldLocationAndRotation (Variables|Default|GetEye) (+ (Transformation|GetWorldLocation (Variables|Default|GetRoombaMesh)) (* (Variables|Default|GetEyeOffset) (Variables|Default|GetScaleMesh))) (Math|Rotator|MakeRotator 0.0 (Variables|Default|GetEyeForwardAngle) 9e+01) false false)
  (Rendering|Lighting|SetOuterConeAngle (Variables|Default|GetEye) (Variables|Default|GetLightWidth)))