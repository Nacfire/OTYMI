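; BP_Multiprise is the actor for the Multiprise object, with a follow camera that becomes the player's view on BeginPlay.
; Each tick, the camera eases toward the closest point on the level's Bp_CameraSpline and looks at the Multiprise.
; The construction script applies mass scale and spring-arm settings.
; Older axis-based camera positioning and plane-locking events, the latter reading the third-person character's YZAxis, remain, but their looping timers are disconnected.
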(event Custom|Camera%20pos
  (bind _multiprise (Variables|Default|GetMultiprise))
  (bind _returnvalue (Transformation|GetWorldLocation _multiprise))
  ;[0.15 0.15 0.15 0.5] Camera Spring Arm
  (if (Variables|Camera|GetInvert%20Camera%20Axis)
    ;;[0.15 0.15 0.15 0.5] Invert X Axis Camera
    (Variables|Camera|SetDistance%20Axis%20Offset (* (Variables|Camera|GetDistance%20From%20Multiprise) 1.0))
    (else
      (Variables|Camera|SetDistance%20Axis%20Offset (* (Variables|Camera|GetDistance%20From%20Multiprise) -1.0))))
  ;;[0.15 0.15 0.15 0.5] Apply Z Offset
  (Variables|/Script/Engine.SpringArmComponent|SetTargetOffset (Variables|Default|GetCamera%20Boom%201) (Math|Vector|MakeVector 0.0 0.0 (Variables|Camera|GetCamera%20Distance%20Z)))
  (if (Variables|Camera|GetIs%20In%20Y%20Axis)
    (Variables|Camera|SetLast%20Pos%20Cam (+ _returnvalue (Math|Vector|MakeVector 0.0 (Variables|Camera|GetDistance%20Axis%20Offset) (Variables|Camera|GetCamera%20Distance%20Z))))
    (else
      (Variables|Camera|SetLast%20Pos%20Cam (+ _returnvalue (Math|Vector|MakeVector (Variables|Camera|GetDistance%20Axis%20Offset) 0.0 (Variables|Camera|GetCamera%20Distance%20Z))))))
  (Transformation|SetActorTransform (Math|Transform|MakeTransform (Variables|Camera|GetLast%20Pos%20Cam) (Math|Rotator|FindRelativeLookatRotation (Math|Transform|MakeTransform (Variables|Camera|GetLast%20Pos%20Cam) "0, 0, 0" "1.000000,1.000000,1.000000") (Transformation|GetWorldLocation (Variables|Default|GetMultiprise))) "1.000000,1.000000,1.000000")))

(event Custom|Reset%20Multiprise%20Pos
  (bind _returnvalue (Transformation|GetActorLocation))
  (bind _returnvalue_2 (Transformation|GetActorLocation))
  ;[0.15 0.15 0.15 0.5] Reset Multiprise Pos
  (if (Variables|/Game/ThirdPerson/Blueprints/BP_ThirdPersonCharacter.BP_ThirdPersonCharacter_C|GetYZ%20Axis (Variables|Default|GetThirdPersonChara%20Ref))
    (Transformation|SetActorLocation self (Math|Vector|MakeVector 0.0 (.y _returnvalue) (.z _returnvalue)) false false)
    (else
      (Transformation|SetActorLocation self (Math|Vector|MakeVector (.x _returnvalue_2) 2e+03 (.z _returnvalue_2)) false false))))

(event EventBeginPlay
  (bind _returnvalue (Actor|GetActorOfClass "/Game/OTYMI/Blueprint/Bp_CameraSpline.Bp_CameraSpline_C"))
  (Variables|Default|SetCamera%20Spline%20BP%20Ref _returnvalue)
  (bind _returnvalue_2 (Actor|GetActorOfClass "/Game/ThirdPerson/Blueprints/BP_ThirdPersonCharacter.BP_ThirdPersonCharacter_C"))
  (Variables|Default|SetThirdPersonChara%20Ref _returnvalue_2)
  (Collision|SetCollisionObjectType (Variables|Default|GetMultiprise) (Variables|Default|GetChannel))
  (Game|Player|SetViewTargetwithBlend (Game|GetPlayerController 0) (Components|GetOwner (Variables|Default|GetFollow%20Camera)) 0.0 "VTBlend_Linear" 0.0 false))

(event EventTick
  (params (DeltaSeconds :type Float%20%28single-precision%29))
  (bind _follow_camera (Variables|Default|GetFollow%20Camera))
  ;[0.15 0.15 0.15 0.5] Update Camera Follow Location Along Spline
  (Transformation|SetWorldLocation _follow_camera (Math|Interpolation|VInterpTo (Transformation|GetWorldLocation (Variables|Default|GetFollow%20Camera)) (Spline|FindLocationClosesttoWorldLocation (Variables|/Game/OTYMI/Blueprint/Bp_CameraSpline.Bp_CameraSpline_C|GetCam%20Spline (Variables|Default|GetCamera%20Spline%20BP%20Ref)) (Transformation|GetWorldLocation (Variables|Default|GetMultiprise)) "World") (Utilities|Time|GetWorldDeltaSeconds) 15.0) false false)
  (Transformation|SetWorldRotation _follow_camera (Math|Rotator|FindLookatRotation (Transformation|GetWorldLocation (Variables|Default|GetFollow%20Camera)) (Transformation|GetWorldLocation (Variables|Default|GetMultiprise))) false false))

(fn ConstructionScript
  (bind _camera_distance_z (Variables|Camera|GetCamera%20Distance%20Z))
  (bind _camera_boom_1 (Variables|Default|GetCamera%20Boom%201))
  (Class|PrimitiveComponent|SetMassScale (Variables|Default|GetMultiprise) "None" (Variables|multiprise|GetPoid))
  (bind _output_get (Variables|/Script/Engine.SpringArmComponent|SetTargetArmLength _camera_boom_1 (Variables|Camera|GetCamera%20X/Y%20Offset)))
  (Variables|/Script/Engine.SpringArmComponent|SetTargetOffset _camera_boom_1 (Math|Vector|MakeVector 0.0 0.0 _camera_distance_z))
  (bind _output_get_2 (Variables|Camera|SetDistance%20Axis%20Offset (* _output_get -1.0)))
  (bind _output_get_3 (Variables|Camera|Setdefault%20Pos%20Cam (+ (Transformation|GetWorldLocation (Variables|Default|GetMultiprise)) (Math|Vector|MakeVector _output_get_2 0.0 _camera_distance_z))))
  (Variables|Camera|SetLast%20Pos%20Cam _output_get_3))