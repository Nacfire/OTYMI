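; BP_OBJWifi is a configurable "Wifi" object that connected players can interact with from within a minimum and maximum distance.
; Connection registers players and runs a looping timer for distance checks, while UnConnect removes them, pauses it and turns the light off.
; Each check colors the point light by range and calls the empty FObjWifi if an in-range player presses interact.
; The construction script applies mesh, material and scale, placing the light above.
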(event Custom|Check_Distance
  (for _array_element (Variables|Default|GetPlayer%20REF%20Array)
    (Variables|Default|SetPlayer%20REF _array_element)
    (if (and (>= (Math|Vector|Distance(Vector) (Transformation|GetActorLocation (Variables|Default|GetPlayer%20REF)) (Transformation|GetActorLocation self)) (Variables|Default|GetMin_distance_to_connect)) (<= (Math|Vector|Distance(Vector) (Transformation|GetActorLocation (Variables|Default|GetPlayer%20REF)) (Transformation|GetActorLocation self)) (Variables|Default|GetMax_distance_to_connect)))
      (Rendering|Components|Light|SetIntensity (Variables|Default|GetPointLight) (Variables|FeedBack|GetIntencity%20light))
      (Rendering|Components|Light|SetLightColor (Variables|Default|GetPointLight) (Variables|FeedBack|GetLight%20Color%20interactible) true)
      (if (Variables|/Game/ThirdPerson/Blueprints/BP_ThirdPersonCharacter.BP_ThirdPersonCharacter_C|GetInteractPress (Variables|Default|GetPlayer%20REF))
        (CallFunction|FObjWifi))
      (else
        (Rendering|Components|Light|SetIntensity (Variables|Default|GetPointLight) (Variables|FeedBack|GetIntencity%20light))
        (Rendering|Components|Light|SetLightColor (Variables|Default|GetPointLight) (Variables|FeedBack|GetLight%20Color%20Uninteractible) true)))))

(event EventBeginPlay)

(event Collision|EventActorBeginOverlap
  (params (OtherActor :type Actor%20Object%20Reference)))

(event EventTick
  (params (DeltaSeconds :type Float%20%28single-precision%29)))

(event EventUnConnect
  (params (Player%20ref :type BP%20Third%20Person%20Character%20Object%20Reference))
  (Utilities|Array|RemoveItem (Variables|Default|GetPlayer%20REF%20Array) Player%20ref)
  (Rendering|Components|Light|SetIntensity (Variables|Default|GetPointLight) 0.0)
  (Utilities|Time|PauseTimerbyHandle (Variables|Default|GetTimerREF)))

(event EventConnection
  (params (PlayerREF :type BP%20Third%20Person%20Character%20Object%20Reference))
  (Utilities|Array|Add (Variables|Default|GetPlayer%20REF%20Array) PlayerREF)
  (if (Utilities|Time|IsValidTimerHandle (Variables|Default|GetTimerREF))
    (Utilities|Time|UnpauseTimerbyHandle (Variables|Default|GetTimerREF))
    (else
      (bind _returnvalue (Utilities|Time|SetTimerbyEvent (delegate Custom|Check_Distance) (Variables|Default|GetTime_entre_2_check_de_distance) true))
      (Variables|Default|SetTimerREF _returnvalue))))

(fn ConstructionScript
  (bind _staticmesh (Variables|Default|GetStaticMesh))
  (bind _mesh (Variables|Default|GetMesh))
  (bind _scale (Variables|Default|GetScale))
  (bind _returnvalue (StaticMesh|GetBoundingBox _mesh))
  (bind _returnvalue_2 (- (.max _returnvalue) (.min _returnvalue)))
  (bind _returnvalue_3 (* _returnvalue_2 _scale))
  (Components|StaticMesh|SetStaticMesh _staticmesh (Variables|Default|GetMesh))
  (Rendering|Material|SetMaterial _staticmesh 0 (Variables|Default|GetMaterial))
  (Transformation|SetWorldScale3D (Variables|Default|GetStaticMesh) (Variables|Default|GetScale))
  (Transformation|SetRelativeLocation (Variables|Default|GetPointLight) (Math|Vector|MakeVector 0.0 0.0 (.Z (Math|Vector|BreakVector (+ _returnvalue_3 (/ _returnvalue_3 2.0))))) false false))

(fn FObjWifi)