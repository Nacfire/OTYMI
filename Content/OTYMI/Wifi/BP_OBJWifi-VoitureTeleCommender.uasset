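; Wifi-connectable actor, named as a remote-controlled car, that moves between its start location and a target actor's location.
; Connection starts or resumes a looping timer, which pauses and triggers the move once a connected player is within the min/max distance range.
; Delayed, rate-adjusted timelines drive opening and closing, chaining when Loop is set.
; Only opening lerps position per update; closing sets it on finish when looping.
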(event Custom|Check_Distance
  (for _array_element (Variables|Default|GetPlayer%20REF%20Array)
    (Variables|Default|SetPlayer%20REF _array_element)
    (if (and (>= (Math|Vector|Distance(Vector) (Transformation|GetActorLocation (Variables|Default|GetPlayer%20REF)) (Transformation|GetActorLocation self)) (Variables|Default|GetMin_distance_to_connect)) (<= (Math|Vector|Distance(Vector) (Transformation|GetActorLocation (Variables|Default|GetPlayer%20REF)) (Transformation|GetActorLocation self)) (Variables|Default|GetMax_distance_to_connect)))
      (CallFunction|FObjWifi)
      (Utilities|Time|PauseTimerbyHandle (Variables|Default|GetTimerREF))
      (if (not (Variables|Voiture|GetIs%20open))
        (Components|Timeline|SetPlayRate (Variables|Default|GetTLOpen) (/ 1.0 (Variables|Voiture|GetTL_OpenRate)))
        (Variables|Voiture|SetIsPlayingTL true)
        (Utilities|FlowControl|Delay (Variables|Voiture|GetWaitBeforeOpen))
        (bind _open_close (Timeline|TLOpen PlayFromStart)
          (:Update
            (Transformation|SetActorLocation (Math|Vector|Lerp(Vector) (Variables|Voiture|GetBaseLocation) (Variables|Voiture|GetFinal_Location) _open_close) false false)
            (Variables|Voiture|SetIsPlayingTL true))
          (:Finished
            (Variables|Voiture|SetIsPlayingTL false)
            (Variables|Voiture|SetIs%20open true)
            (if (Variables|Voiture|GetLoop)
              (CallFunction|PlayStartClose))))))))

(event Custom|PlayStartClose
  (Components|Timeline|SetPlayRate (Variables|Default|GetTLCLose) (/ 1.0 (Variables|Voiture|GetTL_CloseRate)))
  (Variables|Voiture|SetIsPlayingTL true)
  (Utilities|FlowControl|Delay (Variables|Voiture|GetWaitBeforeClose))
  (bind _open_close (Timeline|TLClose PlayFromStart)
    (:Finished
      (Variables|Voiture|SetIsPlayingTL false)
      (Variables|Voiture|SetIs%20open false)
      (if (Variables|Voiture|GetLoop)
        (CallFunction|PlayStartOpen)
        (Transformation|SetActorLocation (Math|Vector|Lerp(Vector) (Variables|Voiture|GetFinal_Location) (Variables|Voiture|GetBaseLocation) _open_close) false false)))))

(event Custom|PlayStartOpen
  (Components|Timeline|SetPlayRate (Variables|Default|GetTLOpen) (/ 1.0 (Variables|Voiture|GetTL_OpenRate)))
  (Variables|Voiture|SetIsPlayingTL true)
  (Utilities|FlowControl|Delay (Variables|Voiture|GetWaitBeforeOpen))
  (bind _open_close (Timeline|TLOpen PlayFromStart)
    (:Update
      (Transformation|SetActorLocation (Math|Vector|Lerp(Vector) (Variables|Voiture|GetBaseLocation) (Variables|Voiture|GetFinal_Location) _open_close) false false)
      (Variables|Voiture|SetIsPlayingTL true))
    (:Finished
      (Variables|Voiture|SetIsPlayingTL false)
      (Variables|Voiture|SetIs%20open true)
      (if (Variables|Voiture|GetLoop)
        (CallFunction|PlayStartClose)))))

(event EventBeginPlay
  (bind _target__location (Variables|Voiture|GetTarget_%20Location))
  (Variables|Voiture|SetBaseLocation (Transformation|GetActorLocation))
  (if (Utilities|IsValid _target__location)
    (Variables|Voiture|SetFinal_Location (Transformation|GetActorLocation _target__location))))

(event EventUnConnect
  (params (Player%20ref :type BP%20Third%20Person%20Character%20Object%20Reference))
  (Utilities|Array|RemoveItem (Variables|Default|GetPlayer%20REF%20Array) Player%20ref)
  (Utilities|Time|PauseTimerbyHandle (Variables|Default|GetTimerREF)))

(event EventConnection
  (params (PlayerREF :type BP%20Third%20Person%20Character%20Object%20Reference))
  (Utilities|Array|Add (Variables|Default|GetPlayer%20REF%20Array) PlayerREF)
  (if (Utilities|Time|IsValidTimerHandle (Variables|Default|GetTimerREF))
    (Utilities|Time|UnpauseTimerbyHandle (Variables|Default|GetTimerREF))
    (else
      (bind _returnvalue (Utilities|Time|SetTimerbyEvent (delegate Custom|Check_Distance) (Variables|Default|GetTime_entre_2_check_de_distance) true))
      (Variables|Default|SetTimerREF _returnvalue))))

(fn ConstructionScript
  (bind _staticmesh (Variables|Default|GetStaticMesh))
  (Components|StaticMesh|SetStaticMesh _staticmesh (Variables|Default|GetMesh))
  (Rendering|Material|SetMaterial _staticmesh 0 (Variables|Default|GetMaterial))
  (Transformation|SetWorldScale3D (Variables|Default|GetStaticMesh) (Variables|Default|GetScale)))

(fn FObjWifi)