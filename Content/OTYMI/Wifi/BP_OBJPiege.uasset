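; BP_OBJPiege is a trap object that reacts to registered players within a minimum and maximum distance band.
; A custom event registers a player and starts or resumes a looping timer that runs Check_Distance on every registered player.
; Players in range are passed to FObjWifi, which is empty here.
; UnConnect removes a player and pauses the shared timer, even if other players remain registered.
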(event Custom|Check_Distance
  (for _array_element (Variables|Default|GetPlayer%20REF%20array)
    (if (Utilities|IsValid _array_element)
      (if (and (>= (Math|Vector|Distance(Vector) (Transformation|GetActorLocation _array_element) (Transformation|GetActorLocation self)) (Variables|Default|GetMin_distance_to_connect)) (<= (Math|Vector|Distance(Vector) (Transformation|GetActorLocation _array_element) (Transformation|GetActorLocation self)) (Variables|Default|GetMax_distance_to_connect)))
        (CallFunction|FObjWifi _array_element)))))

(event Custom|CustomEvent
  (params (PlayerREF :type BP%20Third%20Person%20Character%20Object%20Reference))
  (Utilities|Array|Add (Variables|Default|GetPlayer%20REF%20array) PlayerREF)
  (if (Utilities|Time|IsValidTimerHandle (Variables|Default|GetTimerREF))
    (Utilities|Time|UnpauseTimerbyHandle (Variables|Default|GetTimerREF))
    (else
      (bind _returnvalue (Utilities|Time|SetTimerbyEvent (delegate Custom|Check_Distance) (Variables|Default|GetTime_entre_2_check_de_distance) true))
      (Variables|Default|SetTimerREF _returnvalue))))

(event EventBeginPlay)

(event Collision|EventActorBeginOverlap
  (params (OtherActor :type Actor%20Object%20Reference)))

(event EventTick
  (params (DeltaSeconds :type Float%20%28single-precision%29)))

(event EventUnConnect
  (params (Player%20ref :type BP%20Third%20Person%20Character%20Object%20Reference))
  (Utilities|Array|RemoveItem (Variables|Default|GetPlayer%20REF%20array) Player%20ref)
  (Utilities|Time|PauseTimerbyHandle (Variables|Default|GetTimerREF)))

(fn ConstructionScript)

(fn FObjWifi
  (params (Player%20Ref :type BP%20Third%20Person%20Character%20Object%20Reference)))