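; Wifi switch actor that lets a connected player open or close a linked Door with the DownPress input.
; Connection starts or resumes a looping distance check, paused on UnConnect or beyond twice the player's wifi detection radius.
; Within the min/max connect range, it starts a fast timer polling input to toggle the Door when not animating.
; That input timer is never paused here, and the FObjWifi hook is empty.
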(event Custom|Check%20Input
  ;[0.15 0.15 0.15 0.5] Interupteur
  (if (Variables|/Game/ThirdPerson/Blueprints/BP_ThirdPersonCharacter.BP_ThirdPersonCharacter_C|GetDownPress (Variables|Default|GetPlayer%20REF))
    (if (not (Variables|/Game/OTYMI/Buton_et_interactible/BP_PlatformeMobil.BP_PlatformeMobil_C|GetIsPlayingTL (Variables|Interupteur|GetDoor)))
      (if (Variables|/Game/OTYMI/Buton_et_interactible/BP_PlatformeMobil.BP_PlatformeMobil_C|GetIs%20open (Variables|Interupteur|GetDoor))
        (Class|BPIButontoInterractible|Close(Message) (Variables|Interupteur|GetDoor))
        (else
          (Class|BPIButontoInterractible|Open(Message) (Variables|Interupteur|GetDoor)))))))

(event Custom|Check_Distance
  (if (Utilities|IsValid (Variables|Default|GetPlayer%20REF))
    (if (and (>= (Math|Vector|Distance(Vector) (Transformation|GetActorLocation (Variables|Default|GetPlayer%20REF)) (Transformation|GetActorLocation self)) (Variables|Default|GetMin_distance_to_connect)) (<= (Math|Vector|Distance(Vector) (Transformation|GetActorLocation (Variables|Default|GetPlayer%20REF)) (Transformation|GetActorLocation self)) (Variables|Default|GetMax_distance_to_connect)))
      (CallFunction|FObjWifi)
      ;[0.15 0.15 0.15 0.5] Interupteur
      (if (Utilities|Time|IsValidTimerHandle (Variables|Interupteur|GetTimer%20Check%20to%20open))
        (Utilities|Time|UnpauseTimerbyHandle (Variables|Interupteur|GetTimer%20Check%20to%20open))
        (else
          (bind _returnvalue (Utilities|Time|SetTimerbyEvent (delegate Custom|Check%20Input) 0.01 true true))
          (Variables|Interupteur|SetTimer%20Check%20to%20open _returnvalue)))
      (elif (> (Math|Vector|Distance(Vector) (Transformation|GetActorLocation (Variables|Default|GetPlayer%20REF)) (Transformation|GetActorLocation self)) (* (Variables|/Script/Engine.SphereComponent|GetSphereRadius (Variables|/Game/ThirdPerson/Blueprints/BP_ThirdPersonCharacter.BP_ThirdPersonCharacter_C|GetRange_detection_Wifi (Variables|Default|GetPlayer%20REF))) 2.0))
        (Variables|Default|SetPlayer%20REF 0)
        (Utilities|Time|PauseTimerbyHandle (Variables|Default|GetTimerREF))
        (Development|PrintString "Pause" true true "(R=1.000000,G=0.000000,B=0.000000,A=1.000000)")))))

(event EventBeginPlay)

(event Collision|EventActorBeginOverlap
  (params (OtherActor :type Actor%20Object%20Reference)))

(event EventTick
  (params (DeltaSeconds :type Float%20%28single-precision%29)))

(event EventConnection
  (params (PlayerREF :type BP%20Third%20Person%20Character%20Object%20Reference))
  (Variables|Default|SetPlayer%20REF PlayerREF)
  (if (Utilities|Time|IsValidTimerHandle (Variables|Default|GetTimerREF))
    (Utilities|Time|UnpauseTimerbyHandle (Variables|Default|GetTimerREF))
    (else
      (bind _returnvalue (Utilities|Time|SetTimerbyEvent (delegate Custom|Check_Distance) (Variables|Default|GetTime_entre_2_check_de_distance) true))
      (Variables|Default|SetTimerREF _returnvalue))))

(event EventUnConnect
  (Variables|Default|SetPlayer%20REF 0)
  (Utilities|Time|PauseTimerbyHandle (Variables|Default|GetTimerREF))
  (Development|PrintString "Pause" true true "(R=1.000000,G=0.000000,B=0.000000,A=1.000000)"))

(fn ConstructionScript
  (Components|StaticMesh|SetStaticMesh (Variables|Default|GetStaticMesh) (Variables|Default|GetMesh)))

(fn FObjWifi)