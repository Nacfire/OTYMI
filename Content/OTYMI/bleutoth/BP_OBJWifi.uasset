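; BP_OBJWifi is a Wi-Fi object that holds a connection to a player while that player stays close.
; Connection stores the player reference and starts, or resumes, a looping timer that runs Check_bistance.
; Each check clears the reference and pauses the timer once the player is beyond the minimum connect distance or reaches the maximum, so there is no hysteresis between the two thresholds.
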(event Custom|Check_bistance
  (if (Utilities|IsValid (Variables|Default|GetPlayer%20REF))
    (if (not (and (<= (Math|Vector|Distance(Vector) (Transformation|GetActorLocation (Variables|Default|GetPlayer%20REF)) (Transformation|GetActorLocation self)) (Variables|Default|GetMin_distance_to_connect)) (not (>= (Math|Vector|Distance(Vector) (Transformation|GetActorLocation (Variables|Default|GetPlayer%20REF)) (Transformation|GetActorLocation self)) (Variables|Default|GetMax_distance_to_connect)))))
      (Variables|Default|SetPlayer%20REF 0)
      (Utilities|Time|PauseTimerbyHandle (Variables|Default|GetTimerREF)))))

(event EventBeginPlay)

(event Collision|EventActorBeginOverlap
  (params (OtherActor :type Actor%20Object%20Reference)))

(event EventTick
  (params (DeltaSeconds :type Float%20%28single-precision%29)))

(event EventConnection
  (params (PlayerREF :type BP%20Third%20Person%20Character%20Object%20Reference))
  (Variables|Default|SetPlayer%20REF PlayerREF)
  (if (Utilities|Time|IsValidTimerHandle (Variables|Default|GetTimerREF))
    (Utilities|Time|UnpauseTimerbyHandle (Variables|Default|GetTimerREF))
    (else
      (bind _returnvalue (Utilities|Time|SetTimerbyEvent (delegate Custom|Check_bistance) (Variables|Default|GetTime_entre_2_check_de_distance) true))
      (Variables|Default|SetTimerREF _returnvalue))))

(fn ConstructionScript)